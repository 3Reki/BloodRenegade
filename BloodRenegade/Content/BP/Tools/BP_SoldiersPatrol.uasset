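; BP_SoldiersPatrol is an interactable tool cube, open to all interactors, that steps through how many soldiers in its list are active.
; Each interaction flashes the cube pink, increments the count, then resets and unhides soldiers within it through the AI manager subsystem.
; When the count passes the list length it wraps to one and permanently enables killing of living soldiers beyond the count.
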(event `self.ReceiveBeginPlay`
  (set `/Game/BP/Widgets/WBP_Interact.Letter` "[A]" (cast `/Game/BP/Widgets/WBP_Interact` (`WidgetComponent.GetUserWidgetObject` (`self.Widget`)) :!pure true)))

(event `self.Interact`
  (`self.CubeColor`)
  (`self.Increment Soldier Count`)
  (for (_array_element _array_index) (`self.Soldiers`)
    (if (< _array_index (`self.SoldierCount`))
      (`AIManagerSubsystem.ResetSoldier` (subsystem `AIManagerSubsystem`) _array_element)
      (`self.SetActorHiddenInGame` _array_element false)
      (elif (and (`self.DoKill`) (not (`Soldier.IsDead` _array_element)))
        (`/Game/BP/AI/BP_MySoldier.Die` _array_element)))))

(event `Increment Soldier Count`
  (bind _result (`/Engine/EditorBlueprintResources/StandardMacros.IncrementInt` (`self.SoldierCount`))
    (:`  `
      (if (> _result (`KismetArrayLibrary.Array_Length` (`self.Soldiers`)))
        (set `self.SoldierCount` 1)
        (set `self.DoKill` true)))))

(event `CubeColor`
  (`PrimitiveComponent.SetMaterial` (`self.Cube`) 0 "/Game/GameArt/MasterMaterial/DebugMat/MI_ColorPink.MI_ColorPink")
  (`KismetSystemLibrary.K2_SetTimerDelegate` (delegate `ResetColor`) 0.5))

(event `ResetColor`
  (`PrimitiveComponent.SetMaterial` (`self.Cube`) 0 "/Engine/BasicShapes/BasicShapeMaterial.BasicShapeMaterial"))

(fn `GetWhoCanInteract`
  (returns (ReturnValue :type "EWhoCanInteract Enum"))
  (return "ALL"))

(fn `UserConstructionScript`)