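; BP_SoldierSpawner respawns a referenced Soldier at its starting transform after it dies.
; On BeginPlay it stores the soldier's location and rotation, then starts a looping one-second timer that polls IsDead.
; On death it clears the poll and schedules a delayed respawn, which teleports the soldier back, calls Revive and restarts polling.
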(event `self.ReceiveBeginPlay`
  (bind _soldier (`self.Soldier`))
  (set `self.DefaultLocation` (`self.K2_GetActorLocation` _soldier))
  (set `self.DefaultRotation` (`self.K2_GetActorRotation` _soldier))
  (`self.LaunchTimer`))

(event `LaunchTimer`
  (bind _returnvalue (`KismetSystemLibrary.K2_SetTimerDelegate` (delegate `WaitForRespawn`) 1.0 true)))

(event `WaitForRespawn`
  (if (`Soldier.IsDead` (`self.Soldier`))
    (`KismetSystemLibrary.K2_SetTimerDelegate` (delegate `Respawn`) 5.0)
    (`KismetSystemLibrary.K2_ClearAndInvalidateTimerHandle` (stale `LaunchTimer` _returnvalue))))

(event `Respawn`
  (`self.K2_SetActorLocationAndRotation` (`self.Soldier`) (`self.DefaultLocation`) (`self.DefaultRotation`) false true)
  (`Soldier.Revive` (`self.Soldier`))
  (`self.LaunchTimer`))

(fn `UserConstructionScript`)