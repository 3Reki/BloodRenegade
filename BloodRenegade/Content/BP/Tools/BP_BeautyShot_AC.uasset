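; Actor component, apparently for a beauty shot tool, that tracks a selected camera and can restore its owner's starting transform.
; On BeginPlay it caches the owner's location and rotation, and a reset event teleports the owner back to them.
; Increment and decrement events step an index through the Cameras array with wraparound at both ends.
; GetCurrentCamera returns the camera at that index.
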(event `self.ReceiveBeginPlay`
  (bind _returnvalue (`self.GetOwner`))
  (set `self.InitialLocation` (`Actor.K2_GetActorLocation` _returnvalue))
  (set `self.InitialRotation` (`Actor.K2_GetActorRotation` _returnvalue)))

(event `ResetLocationAndRotation`
  (`Actor.K2_SetActorLocationAndRotation` (`self.GetOwner`) (`self.InitialLocation`) (`self.InitialRotation`) false true))

(event `IncrementIndex`
  (bind _result (`/Engine/EditorBlueprintResources/StandardMacros.IncrementInt` (`self.CurrentIndex`))
    (:`  `
      (if (>= _result (`KismetArrayLibrary.Array_Length` (`self.Cameras`)))
        (set `self.CurrentIndex` 0)))))

(event `DecrementIndex`
  (bind _result (`/Engine/EditorBlueprintResources/StandardMacros.DecrementInt` (`self.CurrentIndex`))
    (:`  `
      (if (< _result 0)
        (set `self.CurrentIndex` (- (`KismetArrayLibrary.Array_Length` (`self.Cameras`)) 1))))))

(fn `GetCurrentCamera`
  (returns (CineCamera :type "CineCameraActor Object Reference"))
  (return (`|GetArrayItem` (`self.Cameras`) (`self.CurrentIndex`))))