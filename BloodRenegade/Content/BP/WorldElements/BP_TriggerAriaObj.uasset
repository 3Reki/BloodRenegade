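; BP_TriggerAriaObj is a one-shot trigger that plays an in-game cinematic and starts an Aria objective.
; On overlap it saves itself as consumed, locks the player and narrows the camera to a cinematic aspect ratio and FOV.
; Chained timelines turn and walk or run the player to a destination while moving the camera.
; Alongside, it destroys any previous Aria and initialises the assigned one at the current checkpoint.
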(event `self.ReceiveBeginPlay`
  (`self.Load`))

(event `self.Box.OnComponentBeginOverlap`
  (params (OverlappedComponent :type "PrimitiveComponent Object Reference") (OtherActor :type "Actor Object Reference") (OtherComp :type "PrimitiveComponent Object Reference") (OtherBodyIndex :type Integer) (bFromSweep :type Boolean) (SweepResult :type "HitResult Structure (by ref)"))
  (bind _asbp_blood_character (cast `/Game/BP/BP_BloodCharacter` OtherActor))
  (`self.Interact` _asbp_blood_character))

(event `Interact`
  (params (Chara :type "BloodCharacter Object Reference"))
  (bind _aria (`self.Aria`))
  (bind (_lastlocation_x _lastlocation_y _lastlocation_z) (`KismetMathLibrary.BreakVector` (`self.LastLocation`)))
  (bind _playerchara (`self.PlayerChara`))
  (bind _playerchara_2 (`self.PlayerChara`))
  (bind _playerchara_3 (`self.PlayerChara`))
  (bind _playerchara_4 (`self.PlayerChara`))
  (bind (_returnvalue_x _returnvalue_y) (`KismetMathLibrary.BreakVector` (`SceneComponent.K2_GetComponentLocation` (`self.PlayerDestination`))))
  (bind _followcamera (`BloodCharacter.FollowCamera` (`self.PlayerChara`)))
  (bind (_returnvalue_roll _returnvalue_pitch _returnvalue_yaw) (`KismetMathLibrary.BreakRotator` (`KismetMathLibrary.FindLookAtRotation` (`self.K2_GetActorLocation` (`self.PlayerChara`)) (`SceneComponent.K2_GetComponentLocation` (`self.PlayerDestination`)))))
  (bind (_returnvalue_location _returnvalue_rotation) (`KismetMathLibrary.BreakTransform` (`SceneComponent.K2_GetComponentToWorld` (`BloodCharacter.FollowCamera` (`self.PlayerChara`)))))
  (if (not (`self.IsConsumed`))
    (bind _asbp_blood_character (cast `/Game/BP/BP_BloodCharacter` Chara))
    (set `self.PlayerChara` _asbp_blood_character)
    (set `self.IsConsumed` true)
    (message `/Game/BP/SaveSystem/BPI_Saver.SaveConsumable` (`GameplayStatics.GetGameInstance`) (`KismetSystemLibrary.GetObjectName` self) false)
    (`BloodCharacter.SetCrouch` _playerchara_3 false)
    ;[1 1 1] Reset Player Camera
    (`BloodCharacter.SetCantMove` _playerchara_3 true)
    (`PrimitiveComponent.SetCollisionEnabled` (`self.Box`) "NoCollision")
    (bind _output_get (set `self.StartAspectRatio` (`CameraComponent.AspectRatio` _followcamera)))
    (bind (_direction _lerp) (`Timeline|Timeline_0` :!via `PlayFromStart`)
      (:`Update`
        (`CameraComponent.SetAspectRatio` _followcamera (`KismetMathLibrary.Lerp` _output_get 2.4 _lerp))
        (`CameraComponent.SetFieldOfView` _followcamera (`KismetMathLibrary.Lerp` 90.0 55.0 _lerp)))
      (:`Finished`
        (set `self.LastRotation` (`self.K2_GetActorRotation` (`self.PlayerChara`)))
        (set `self.NextRotation` (`KismetMathLibrary.MakeRotator` 0.0 0.0 _returnvalue_yaw))
        (bind (_direction_2 _lerp_2) (`Timeline|Timeline_1` :!via `PlayFromStart`)
          (:`Update`
            (`self.K2_SetActorRotation` _playerchara (`KismetMathLibrary.RLerp` (`self.LastRotation`) (`self.NextRotation`) _lerp_2 true) false))
          (:`Finished`
            (`/Game/BP/BP_BloodCharacter.ResetCameraFocus` _playerchara)
            (`KismetSystemLibrary.Delay` 0.3)
            (set `self.LastCamRotation` _returnvalue_rotation)
            ;[1 1 1] Set Camera For Cinématique
            (set `self.LastCamLocation` _returnvalue_location)
            (set `self.LastLocation` (`self.K2_GetActorLocation` _playerchara_4))
            (set `self.LastRotation` (`self.K2_GetActorRotation` _playerchara_4))
            (if (`self.IsIseraRunning`)
              (`Character.PlayAnimMontage` _playerchara_2 "/Game/GameArt/Animation/Montage/A_Run_Montage.A_Run_Montage" 0.5 "None")
              (else
                (`Character.PlayAnimMontage` _playerchara_2 "/Game/GameArt/Animation/Montage/A_Walk_Montage.A_Walk_Montage" 0.5 "None")))
            (`|ExecutionSequence`
              (:`then_0`
                (`TimelineComponent.SetPlayRate` (`self.Timeline`) (`self.IseraSpeed`))
                (bind (_direction_3 _lerpplayer _lerpplayerrota _lerpcampos _lerpcamrota) (`Timeline|Timeline` :!via `PlayFromStart`)
                  (:`Update`
                    (`|ExecutionSequence`
                      (:`then_0`
                        (`self.K2_SetActorLocationAndRotation` (`self.PlayerChara`) (`KismetMathLibrary.VLerp` (`self.LastLocation`) (`KismetMathLibrary.MakeVector` _returnvalue_x _returnvalue_y _lastlocation_z) _lerpplayer) (`KismetMathLibrary.RLerp` (`self.LastRotation`) (`SceneComponent.K2_GetComponentRotation` (`self.PlayerDestination`)) _lerpplayerrota true) false false))
                      (:`then_1`
                        (`SceneComponent.K2_SetWorldLocationAndRotation` (`BloodCharacter.FollowCamera` (`self.PlayerChara`)) (`KismetMathLibrary.VLerp` (`self.LastCamLocation`) (`self.CamLocation`) _lerpcampos) (`KismetMathLibrary.RLerp` (`self.LastCamRotation`) (`self.CamRocation`) _lerpcamrota true) false false))))
                  (:`Finished`
                    (`Character.PlayAnimMontage` (`self.PlayerChara`) "/Game/GameArt/Animation/Montage/A_Idle_Montage.A_Idle_Montage" 1.0 "None"))))
              (:`then_1`
                (if (`KismetSystemLibrary.IsValidSoftObjectReference` (`self.LastAria`))
                  (`AriaObjectif.SetActiveEscort` (`|ConvertAsset` (`self.LastAria`)) (`self.PlayerChara`) false)
                  (if (`self.BlockingCharacter`)
                    (`BloodCharacter.SetCantMove` (`self.PlayerChara`) true))
                  (`self.K2_DestroyActor` (`|ConvertAsset` (`self.LastAria`))))
                (`/Engine/EditorBlueprintResources/StandardMacros.IsValid` _aria
                  (:`Is Valid`
                    (`AriaObjectif.InitAria` _aria (`self.PlayerChara`))
                    (`AriaObjectif.SetCurrentObj` _aria (`self.CurrentCheckpoint`))
                    (`AriaObjectif.StartObject` _aria)))))))))))

(fn `Load`
  (bind (_savegamedata _saveexists) (message `/Game/BP/SaveSystem/BPI_Saver.GetSaveData` (`GameplayStatics.GetGameInstance`)))
  (if _saveexists
    (set `self.IsConsumed` (`BlueprintSetLibrary.Set_Contains` (`/Game/BP/SaveSystem/BP_SaveGame.Consumables` _savegamedata) (`KismetSystemLibrary.GetObjectName` self)))
    (return)
    (else
      (return))))

(fn `UserConstructionScript`)