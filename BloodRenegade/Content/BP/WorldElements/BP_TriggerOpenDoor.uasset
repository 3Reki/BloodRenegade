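; BP_TriggerOpenDoor is a one-shot trigger box that switches on a linked Door when the blood character overlaps it.
; The first interaction marks it consumed, saves its object name as a consumable without flushing, then switches the door on after a delay.
; On BeginPlay, Load restores the consumed flag from save data and switches the door on whenever a save exists, regardless of that flag.
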(event `self.ReceiveBeginPlay`
  (`self.Load`))

(event `self.Box.OnComponentBeginOverlap`
  (params (OverlappedComponent :type "PrimitiveComponent Object Reference") (OtherActor :type "Actor Object Reference") (OtherComp :type "PrimitiveComponent Object Reference") (OtherBodyIndex :type Integer) (bFromSweep :type Boolean) (SweepResult :type "HitResult Structure (by ref)"))
  (bind _asbp_blood_character (cast `/Game/BP/BP_BloodCharacter` OtherActor))
  (`self.Interact` _asbp_blood_character))

(event `Interact`
  (params (Chara :type "BloodCharacter Object Reference"))
  (if (not (`self.IsConsumed`))
    (bind _asbp_blood_character (cast `/Game/BP/BP_BloodCharacter` Chara))
    (set `self.PlayerChara` _asbp_blood_character)
    (set `self.IsConsumed` true)
    (message `/Game/BP/SaveSystem/BPI_Saver.SaveConsumable` (`GameplayStatics.GetGameInstance`) (`KismetSystemLibrary.GetObjectName` self) false)
    (`KismetSystemLibrary.Delay` 7.5)
    (`MotherWorldElements.SwitchOn` (`|ConvertAsset` (`self.Door`)))))

(fn `Load`
  (bind (_savegamedata _saveexists) (message `/Game/BP/SaveSystem/BPI_Saver.GetSaveData` (`GameplayStatics.GetGameInstance`)))
  (if _saveexists
    (set `self.IsConsumed` (`BlueprintSetLibrary.Set_Contains` (`/Game/BP/SaveSystem/BP_SaveGame.Consumables` _savegamedata) (`KismetSystemLibrary.GetObjectName` self)))
    (`MotherWorldElements.SwitchOn` (`|ConvertAsset` (`self.Door`)))
    (return)
    (else
      (return))))

(fn `UserConstructionScript`)