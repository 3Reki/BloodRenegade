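; BP_ObjectiveTarget is a world objective marker that shows a widget and sets the current objective text on the BloodHUD.
; On BeginPlay it enables itself if its object name matches the saved objective, or if it is flagged as the first objective when no save exists.
; Enabling also records its object name through the game instance without flushing the save, while disabling only hides the widget.
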(event `self.ReceiveBeginPlay`
  (bind (_savegamedata _saveexists) (message `/Game/BP/SaveSystem/BPI_Saver.GetSaveData` (`GameplayStatics.GetGameInstance`)))
  (if _saveexists
    (if (`KismetStringLibrary.EqualEqual_StrStr` (`KismetSystemLibrary.GetObjectName` self) (`/Game/BP/SaveSystem/BP_SaveGame.Objective` _savegamedata))
      (`self.Enable` :!label _label))
    (elif (`self.FirstObjective`)
      (goto _label))))

(event `Enable`
  (`SceneComponent.SetHiddenInGame` (`self.Widget`) false false)
  (`BloodHUD.SetObjectiveText` (cast `BloodHUD` (`PlayerController.GetHUD` (`GameplayStatics.GetPlayerController` 0)) :!pure true) (`self.ObjectiveName`))
  (message `/Game/BP/SaveSystem/BPI_Saver.SaveObjective` (`GameplayStatics.GetGameInstance`) (`KismetSystemLibrary.GetObjectName` self) false))

(event `Disable`
  (`SceneComponent.SetHiddenInGame` (`self.Widget`) true false))

(fn `UserConstructionScript`)