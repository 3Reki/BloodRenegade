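; BP_SearchingLampUV is a lamp, named as a UV searching light, that switches on and off and can show a blinded effect.
; Switch-on flickers the light up to its stored intensity through a timeline paced by the data asset's blinking period, then enables overlap events on its mesh collider.
; Switch-off saves the intensity, hides the light and disables overlaps.
; BlindEffect toggles the affected-lamp effect, and GetBlindOffset returns a constant.
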(event `self.SwitchOn`
  (bind _lightsource (`self.LightSource`))
  (`LightComponent.SetIntensity` _lightsource 0.0)
  (`SceneComponent.SetVisibility` _lightsource true false)
  (`TimelineComponent.SetPlayRate` (`self.SwitchOnFlick`) (`LampUVDataAsset.BlinkingPeriod` (`self.DataAsset`)))
  (bind (_direction _lerp) (`Timeline|SwitchOnFlick` :!via `PlayFromStart`)
    (:`Update`
      (`LightComponent.SetIntensity` (`self.LightSource`) (* _lerp (`self.Intensity`))))
    (:`Finished`
      (set `PrimitiveComponent.bGenerateOverlapEvents` true (`self.MeshCollider`)))))

(event `self.SwitchOff`
  (set `self.Intensity` (`LightComponentBase.Intensity` (`self.LightSource`)))
  (`SceneComponent.SetVisibility` (`self.LightSource`) false false)
  (set `PrimitiveComponent.bGenerateOverlapEvents` false (`self.MeshCollider`)))

(event `self.BlindEffect`
  (params (b :type Boolean))
  (bind _ns_affectedlamp (`self.NS_AffectedLamp`))
  (if b
    (`ActorComponent.Activate` _ns_affectedlamp true)
    (else
      (`ActorComponent.Deactivate` _ns_affectedlamp))))

(fn `GetBlindOffset`
  (returns (ReturnValue :type "Float (single-precision)"))
  (return 40.0))

(fn `UserConstructionScript`)