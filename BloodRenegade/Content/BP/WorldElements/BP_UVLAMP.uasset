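; BP_UVLAMP is a switchable UV lamp world element that can show a blind effect through NSAffectedLamp.
; Switching on plays a flicker timeline at a data-asset rate, driving light intensity and emissive-style custom primitive data, then enables mesh overlap events.
; Switching off saves the intensity for the next flicker, hides lights and flares, disables overlaps and optionally posts a Wwise sound.
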(event `self.SwitchOn`
  (`LightComponent.SetIntensity` (`self.LightSource`) 0.0)
  (`SceneComponent.SetVisibility` (`self.LightSource`) true false)
  (`SceneComponent.SetVisibility` (`self.Flare2`) true false)
  (`SceneComponent.SetVisibility` (`self.SoftLight`) true false)
  (`SceneComponent.SetVisibility` (`self.Flare1`) true false)
  (`TimelineComponent.SetPlayRate` (`self.SwitchOnFlick`) (`LampUVDataAsset.BlinkingPeriod` (`self.DataAsset`)))
  (bind (_direction _lerp) (`Timeline|SwitchOnFlick` :!via `PlayFromStart`)
    (:`Update`
      (`PrimitiveComponent.SetCustomPrimitiveDataFloat` (`self.MeshCollider`) 0 _lerp)
      (`LightComponent.SetIntensity` (`self.LightSource`) (* _lerp (`self.Intensity`))))
    (:`Finished`
      (set `PrimitiveComponent.bGenerateOverlapEvents` true (`self.MeshCollider`)))))

(event `self.BlindEffect`
  (params (b :type Boolean))
  (bind _ns_affectedlamp (`self.NS_AffectedLamp`))
  (if b
    (`ActorComponent.Activate` _ns_affectedlamp true)
    (else
      (`ActorComponent.Deactivate` _ns_affectedlamp))))

(event `self.SwitchOff`
  (set `self.Intensity` (`LightComponentBase.Intensity` (`self.LightSource`)))
  (`SceneComponent.SetVisibility` (`self.LightSource`) false false)
  (`SceneComponent.SetVisibility` (`self.Flare2`) false false)
  (`SceneComponent.SetVisibility` (`self.SoftLight`) false false)
  (`SceneComponent.SetVisibility` (`self.Flare1`) false false)
  (set `PrimitiveComponent.bGenerateOverlapEvents` false (`self.MeshCollider`))
  (`PrimitiveComponent.SetCustomPrimitiveDataFloat` (`self.MeshCollider`) 0 0.0)
  (if (`self.PlaySound`)
    (`AkGameplayStatics.PostEvent` "/Game/WwiseAudio/Events/Environment_Work_Unit/SFX_SolarLight_TurnOff.SFX_SolarLight_TurnOff" self)))

(fn `GetBlindOffset`
  (returns (ReturnValue :type "Float (single-precision)"))
  (return 20.0))

(fn `UserConstructionScript`)