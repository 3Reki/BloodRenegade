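; Scripted Aria character that runs objective actions such as spawning, dialogue, generator use, escort activation and deletion, around cutscene-like moments with the player.
; ExecutAction dispatches each action, with most waiting a per-point delay before calling NextObjectif.
; Timelines with runtime-swapped curves drive mouth animation and emotion morph targets, and dialogue advances to a second set after playing.
; ResetCam blends the player's follow camera transform, aspect ratio and FOV back to gameplay values.
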(event `self.InitAria`
  (params (Chara :type "BloodCharacter Object Reference"))
  (set `self.PlayerChara` (`|ConvertAsset` (cast `/Game/BP/BP_BloodCharacter` Chara :!pure true)))
  (set `self.CurrentDialogue` (`self.BP_Dialogue_AC`))
  (set `self.CurentDialogueAriaMouthCurve` (`self.Dialogue1AriaMouthCurve`)))

(event `self.ExecutAction`
  (params (Action :type "EAriaActions Enum" :default "DeleteAria"))
  (bind _dialoguetimeline (`self.DialogueTImeline`))
  (bind _curentdialogueariamouthcurve (`self.CurentDialogueAriaMouthCurve`))
  (bind _output (`|ConvertAsset` (`self.PlayerChara`)))
  (bind _output_2 (`|ConvertAsset` (`self.PlayerChara`)))
  (switch `EAriaActions` Action
    (:`DeleteAria`
      (`self.NextObjectif`)
      (`self.K2_DestroyActor`))
    (:`SpawnAria`
      (`SceneComponent.SetVisibility` (`self.SkeletalMesh`) true false)
      (bind _returnvalue (`self.GetTimingWithPoint`))
      (`KismetSystemLibrary.Delay` _returnvalue)
      (`self.NextObjectif`))
    (:`ReAbleMovementPlayer`
      (`AkGameplayStatics.SetState` "/Game/WwiseAudio/States/Default_Work_Unit/Music_State/Music_State-InGame.Music_State-InGame")
      (`BloodCharacter.SetCantMove` _output_2 false)
      (`SkeletalMeshComponent.SetAnimationMode` (`Character.Mesh` _output_2) "AnimationBlueprint")
      (`self.ResetCam`)
      (bind _returnvalue_2 (`self.GetTimingWithPoint`))
      (`KismetSystemLibrary.Delay` _returnvalue_2)
      (`self.NextObjectif`))
    (:`PlayDialogue`
      (`/Game/BP/Interactable/BP_Dialogue_AC.PlayDialogue` (`self.CurrentDialogue`))
      (`TimelineComponent.SetFloatCurve` _dialoguetimeline _curentdialogueariamouthcurve "AriaMouth")
      (`TimelineComponent.SetTimelineLength` _dialoguetimeline (`.MaxTime` (`CurveBase.GetTimeRange` _curentdialogueariamouthcurve)))
      (`|ExecutionSequence`
        (:`then_0`
          (bind _returnvalue_3 (`self.GetTimingWithPoint` :!label _label))
          (`KismetSystemLibrary.Delay` _returnvalue_3)
          (`self.NextObjectif`))
        (:`then_1`
          (bind (_direction _ariamouth) (`Timeline|DialogueTImeline` :!via `PlayFromStart`)
            (:`Update`
              (set `self.Aria Mouth` _ariamouth))
            (:`Finished`
              (set `self.CurrentDialogue` (`self.BP_Dialogue_AC2`))
              (set `self.CurentDialogueAriaMouthCurve` (`self.Dialogue2AriaMouthCurve`)))))))
    (:`MoveToNextPoint`
      (goto _label))
    (:`SetActiveEscort`
      (`SkeletalMeshComponent.SetAnimationMode` (`Character.Mesh` _output) "AnimationBlueprint")
      (`self.SetActiveEscort` _output true)
      (`SkeletalMeshComponent.SetAnimationMode` (`self.SkeletalMesh`) "AnimationBlueprint")
      (`self.ResetCam`))
    (:`ResetPlayerCamera`
      (`|ExecutionSequence`
        (:`then_0`
          (`self.ResetCam`))
        (:`then_1`
          (bind _returnvalue_4 (`self.GetTimingWithPoint`))
          (`KismetSystemLibrary.Delay` _returnvalue_4)
          (`self.NextObjectif`))))
    (:`UseGenerator`
      (`IInteractable.Interact` (cast `/Game/BP/Interactable/BP_Switch` (`|ConvertAsset` (`self.CurrentGenerator`)) :!pure true))
      (bind _returnvalue_5 (`self.GetTimingWithPoint`))
      (`KismetSystemLibrary.Delay` _returnvalue_5)
      (`self.NextObjectif`))))

(event `ResetCam`
  (bind _output (`|ConvertAsset` (`self.PlayerChara`)))
  (bind _followcamera (`BloodCharacter.FollowCamera` _output))
  (bind _followcamera_2 (`BloodCharacter.FollowCamera` _output))
  (`|ExecutionSequence`
    (:`then_0`
      (set `self.CamLocation` (`SceneComponent.RelativeLocation` _followcamera_2))
      (set `self.CamRocation` (`SceneComponent.RelativeRotation` _followcamera_2))
      (bind (_direction _lerp) (`Timeline|ResetCameraPlayer` :!via `PlayFromStart`)
        (:`Update`
          (`SceneComponent.K2_SetRelativeLocationAndRotation` _followcamera_2 (`KismetMathLibrary.VLerp` (`self.CamLocation`) (0.0 0.0 0.0) _lerp) (`KismetMathLibrary.RLerp` (`self.CamRocation`) (struct) _lerp true) false false))))
    (:`then_1`
      (bind _output_get (set `self.LastPlayerAspectRatio` (`CameraComponent.AspectRatio` _followcamera)))
      (bind (_direction_2 _lerp_2) (`Timeline|Timeline` :!via `PlayFromStart`)
        (:`Update`
          (`CameraComponent.SetAspectRatio` (`BloodCharacter.FollowCamera` _output) (`KismetMathLibrary.Lerp` _output_get 1.777778 _lerp_2))
          (`CameraComponent.SetFieldOfView` _followcamera (`KismetMathLibrary.Lerp` 55.0 90.0 _lerp_2)))))))

(event `self.StartEmotionTimeline`
  (bind _skeletalmesh (`self.SkeletalMesh`))
  (bind _timelineemotions (`self.TimelineEmotions`))
  (bind _curveemotions (`self.CurveEmotions`))
  (`TimelineComponent.SetVectorCurve` _timelineemotions _curveemotions "BlendShapes")
  (`TimelineComponent.SetTimelineLength` _timelineemotions (`.MaxTime` (`CurveBase.GetTimeRange` _curveemotions)))
  (bind (_direction _blendshapes) (`Timeline|TimelineEmotions` :!via `PlayFromStart`)
    (:`Update`
      (bind (_x _y _z) (`KismetMathLibrary.BreakVector3f` _blendshapes))
      (`SkeletalMeshComponent.SetMorphTarget` _skeletalmesh "Happy" _x true)
      (`SkeletalMeshComponent.SetMorphTarget` _skeletalmesh "Fear_0" _y true)
      (`SkeletalMeshComponent.SetMorphTarget` _skeletalmesh "Sad" _z true))))

(fn `ResetAspectRatio`)

(fn `ResetCameraPositionPlayer`)

(fn `UserConstructionScript`)