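; Spline actor that places a row of hook points along its path, built at construction time.
; The construction script calls CreateHooks, which adds scaled-down child actors from an Offset start, stepped by Padding until the spline length is exceeded.
; Each position is the distance divided by spline length, sampled in local space at constant velocity for even spacing.
; The event graph holds no runtime logic.
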(fn `CreateHooks`
  (locals (HookCount :type Integer))
  (bind _spline (`self.Spline`))
  (bind _returnvalue (/ (+ (`self.Offset`) (* (`self.Padding`) (`local.HookCount`))) (`SplineComponent.GetSplineLength` _spline)))
  (while (<= _returnvalue 1.0)
    (`AddComponent|NODE_AddChildActorComponent-5` :`RelativeTransform` (`KismetMathLibrary.MakeTransform` (`SplineComponent.GetLocationAtTime` _spline _returnvalue "Local" true) (struct) (0.2 0.2 0.2)))
    (`/Engine/EditorBlueprintResources/StandardMacros.IncrementInt` (`local.HookCount`))))

(fn `UserConstructionScript`
  (`self.CreateHooks`))