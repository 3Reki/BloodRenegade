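; World trigger volume that fades a rich text widget on screen while the player character (BP_BloodCharacter) is inside its box.
; BeginPlay creates the widget from the formatted Text and input replace strings.
; On overlap, if the subtitles setting is enabled, it adds the widget to the viewport and plays an opacity timeline.
; Leaving reverses the timeline, removing the widget once the fade-out finishes.
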(event `self.ReceiveBeginPlay`
  (bind _returnvalue (`|CreateWidget` "/Game/BP/Widgets/WBP_RichText.WBP_RichText_C" null (`|FormatText` (`self.Text`) " \n" _) (`self.InputReplaceStrings`)))
  (set `self.Widget` _returnvalue)
  (set `PrimitiveComponent.bGenerateOverlapEvents` true (`self.Box`)))

(event `self.Box.OnComponentBeginOverlap`
  (params (OverlappedComponent :type "PrimitiveComponent Object Reference") (OtherActor :type "Actor Object Reference") (OtherComp :type "PrimitiveComponent Object Reference") (OtherBodyIndex :type Integer) (bFromSweep :type Boolean) (SweepResult :type "HitResult Structure (by ref)"))
  (bind _widget (`self.Widget`))
  (bind _widget_2 (`self.Widget`))
  (cast `/Game/BP/BP_BloodCharacter` OtherActor)
  (bind _returnvalue (`BloodGameUserSettings.GetBloodGameUserSettings`))
  (if (`BloodGameUserSettings.DisplaySubtitles` _returnvalue)
    (if (`Widget.IsInViewport` _widget_2)
      (bind (_direction _opacity) (`Timeline|OpacityTimeline` :!label _label)
        (:`Update`
          (`Widget.SetRenderOpacity` _widget _opacity))
        (:`Finished`
          (switch `ETimelineDirection` _direction
            (:`Backward`
              (`Widget.RemoveFromParent` _widget)))))
      (else
        (`UserWidget.AddToViewport` _widget_2 0)
        (goto _label)))))

(event `self.Box.OnComponentEndOverlap`
  (params (OverlappedComponent :type "PrimitiveComponent Object Reference") (OtherActor :type "Actor Object Reference") (OtherComp :type "PrimitiveComponent Object Reference") (OtherBodyIndex :type Integer))
  (cast `/Game/BP/BP_BloodCharacter` OtherActor)
  (if (`Widget.IsInViewport` (`self.Widget`))
    (goto _label :!via `Reverse`)))

(fn `UserConstructionScript`)