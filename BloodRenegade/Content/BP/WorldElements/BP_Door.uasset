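; Switchable path-blocker door that starts on or off per IsOn, with Wwise presence audio near the player and a deactivation sound.
; Construction script scales the blocker, builds instanced pillar stacks on both sides from DoorScale, and applies the initial state.
; SwitchOff and Switchon play or reverse one timeline, fading blocker and pillar lights through custom primitive data.
; Visibility, collision and point light update when the timeline finishes.
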(event `self.ReceiveBeginPlay`
  (if (< (`KismetMathLibrary.Vector_DistanceSquared` (`self.K2_GetActorLocation` (`GameplayStatics.GetPlayerCharacter` 0)) (`SceneComponent.K2_GetComponentLocation` (`self.Box`))) (`KismetMathLibrary.Square` (`SphereComponent.SphereRadius` (`self.SoundSphere`))))
    (`AkGameObject.PostAkEvent` :`self` (`self.Ak`) :`AkEvent` "/Game/WwiseAudio/Events/Environment_Work_Unit/SFX_PathBlocker_Presence.SFX_PathBlocker_Presence")))

(event `self.SwitchOff`
  (bind _box (`self.Box`))
  (bind _sm_doorpathblocker (`self.SM_DoorPathBlocker`))
  (bind _sm_doorpathblocker_2 (`self.SM_DoorPathBlocker`))
  (set `self.IsOn` false)
  (`AkGameObject.PostAkEvent` :`self` (`self.Ak`) :`AkEvent` "/Game/WwiseAudio/Events/Environment_Work_Unit/SFX_PathBlocker_Desactivation.SFX_PathBlocker_Desactivation")
  (set `self.ColliderEnabler` false)
  (bind (_direction _open _lightsoff) (`Timeline|Open Timeline` :!label _label)
    (:`Update`
      (`PrimitiveComponent.SetCustomPrimitiveDataFloat` (`self.SM_DoorPathBlocker`) 0 _open)
      (`PrimitiveComponent.SetCustomPrimitiveDataFloat` (`self.TopPillar`) 0 _lightsoff)
      (`PrimitiveComponent.SetCustomPrimitiveDataFloat` (`self.MidPillar`) 0 _lightsoff)
      (`PrimitiveComponent.SetCustomPrimitiveDataFloat` (`self.BottomPillar`) 0 _lightsoff))
    (:`Finished`
      (if (`self.ColliderEnabler`)
        (`SceneComponent.SetHiddenInGame` _sm_doorpathblocker false false)
        (`PrimitiveComponent.SetCollisionEnabled` _sm_doorpathblocker_2 "QueryOnly")
        (`PrimitiveComponent.SetCollisionEnabled` _box "QueryAndPhysics")
        (`LightComponent.SetIntensity` (`self.PointLight`) 2000.0)
        (else
          (`SceneComponent.SetHiddenInGame` _sm_doorpathblocker true false)
          (`PrimitiveComponent.SetCollisionEnabled` _sm_doorpathblocker_2 "NoCollision")
          (`PrimitiveComponent.SetCollisionEnabled` _box "NoCollision")
          (`LightComponent.SetIntensity` (`self.PointLight`) 0.0))))))

(event `self.SwitchOn`
  (set `self.IsOn` true)
  (set `self.ColliderEnabler` true)
  (goto _label :!via `Reverse`))

(event `self.SoundSphere.OnComponentBeginOverlap`
  (params (OverlappedComponent :type "PrimitiveComponent Object Reference") (OtherActor :type "Actor Object Reference") (OtherComp :type "PrimitiveComponent Object Reference") (OtherBodyIndex :type Integer) (bFromSweep :type Boolean) (SweepResult :type "HitResult Structure (by ref)"))
  (if (`self.IsOn`)
    (cast `/Game/BP/BP_BloodCharacter` OtherActor)
    (`AkGameObject.PostAkEvent` :`self` (`self.Ak`) :`AkEvent` "/Game/WwiseAudio/Events/Environment_Work_Unit/SFX_PathBlocker_Presence.SFX_PathBlocker_Presence")))

(event `self.SoundSphere.OnComponentEndOverlap`
  (params (OverlappedComponent :type "PrimitiveComponent Object Reference") (OtherActor :type "Actor Object Reference") (OtherComp :type "PrimitiveComponent Object Reference") (OtherBodyIndex :type Integer))
  (if (`self.IsOn`)
    (cast `/Game/BP/BP_BloodCharacter` OtherActor)
    (`AkGameObject.Stop` (`self.Ak`))))

(fn `GetOffset`
  (returns (ReturnValue :type "Float (single-precision)"))
  (return 0.0))

(fn `GetWhoCanInteract`
  (returns (ReturnValue :type "EWhoCanInteract Enum"))
  (return "ALL"))

(fn `UserConstructionScript`
  (bind _box (`self.Box`))
  (bind _sm_doorpathblocker (`self.SM_DoorPathBlocker`))
  (bind _sm_doorpathblocker_2 (`self.SM_DoorPathBlocker`))
  (bind (_x _y _z) (`KismetMathLibrary.BreakVector3f` (`self.DoorScale`)))
  (bind (_x_2 _y_2 _z_2) (`KismetMathLibrary.BreakVector3f` (`self.DoorScale`)))
  ;[1 1 1] Scale
  (`SceneComponent.SetWorldScale3D` (`self.SM_DoorPathBlocker`) (`self.DoorScale`))
  (`TimelineComponent.SetPlayRate` (`self.Open Timeline`) (/ 1.0 (`self.Open Length`)))
  (`|ExecutionSequence`
    (:`then_0`
      ;[1 1 1] Base
      (`InstancedStaticMeshComponent.AddInstance` (`self.BottomPillar`) (`KismetMathLibrary.MakeTransform` (`KismetMathLibrary.MakeVector` (/ (* (`KismetMathLibrary.BreakVector3f` (`self.DoorScale`)) -100.0) 2.0))) false)
      ;[1 1 1] MidPillar
      (for _index (range (+ (`KismetMathLibrary.FTrunc` (- (`.Z` (`KismetMathLibrary.BreakVector3f` (`self.DoorScale`))) 4.0)) 1))
        (`InstancedStaticMeshComponent.AddInstance` (`self.MidPillar`) (`KismetMathLibrary.MakeTransform` (`KismetMathLibrary.MakeVector` (/ (* (`KismetMathLibrary.BreakVector3f` (`self.DoorScale`)) -100.0) 2.0) 0.0 (+ 200.0 (* _index (`.Z` (`KismetMathLibrary.BreakVector3f` (`.Max` (`StaticMeshComponent.GetLocalBounds` (`self.MidPillar`))))))))) false)
        ;[1 1 1] EndPillar
        (`InstancedStaticMeshComponent.AddInstance` (`self.TopPillar`) (`KismetMathLibrary.MakeTransform` (`KismetMathLibrary.MakeVector` (/ (* _x_2 -100.0) 2.0) 0.0 (- (* _z_2 100.0) (`.Z` (`KismetMathLibrary.BreakVector3f` (`.Max` (`StaticMeshComponent.GetLocalBounds` (`self.TopPillar`)))))))) false)))
    (:`then_1`
      ;[1 1 1] Base
      (`InstancedStaticMeshComponent.AddInstance` (`self.BottomPillar`) (`KismetMathLibrary.MakeTransform` (`KismetMathLibrary.MakeVector` (/ (* (`KismetMathLibrary.BreakVector3f` (`self.DoorScale`)) 100.0) 2.0)) (struct :`Yaw` 180.0)) false)
      ;[1 1 1] MidPillar
      (for _index_2 (range (+ (`KismetMathLibrary.FTrunc` (- (`.Z` (`KismetMathLibrary.BreakVector3f` (`self.DoorScale`))) 4.0)) 1))
        (`InstancedStaticMeshComponent.AddInstance` (`self.MidPillar`) (`KismetMathLibrary.MakeTransform` (`KismetMathLibrary.MakeVector` (/ (* (`KismetMathLibrary.BreakVector3f` (`self.DoorScale`)) 100.0) 2.0) 0.0 (+ 200.0 (* _index_2 (`.Z` (`KismetMathLibrary.BreakVector3f` (`.Max` (`StaticMeshComponent.GetLocalBounds` (`self.MidPillar`)))))))) (struct :`Yaw` 180.0)) false)
        ;[1 1 1] EndPillar
        (`InstancedStaticMeshComponent.AddInstance` (`self.TopPillar`) (`KismetMathLibrary.MakeTransform` (`KismetMathLibrary.MakeVector` (/ (* _x 100.0) 2.0) 0.0 (- (* _z 100.0) (`.Z` (`KismetMathLibrary.BreakVector3f` (`.Max` (`StaticMeshComponent.GetLocalBounds` (`self.TopPillar`))))))) (struct :`Yaw` 180.0)) false)))
    (:`then_2`
      (if (`self.IsOn`)
        (`SceneComponent.SetHiddenInGame` _sm_doorpathblocker false false)
        (`PrimitiveComponent.SetCollisionEnabled` _sm_doorpathblocker_2 "QueryOnly")
        (`PrimitiveComponent.SetCollisionEnabled` _box "QueryAndPhysics")
        (`LightComponent.SetIntensity` (`self.PointLight`) 2000.0)
        (`PrimitiveComponent.SetCustomPrimitiveDataFloat` (`self.SM_DoorPathBlocker`) 0 0.0)
        (`PrimitiveComponent.SetCustomPrimitiveDataFloat` (`self.TopPillar`) 0 1.0)
        (`PrimitiveComponent.SetCustomPrimitiveDataFloat` (`self.MidPillar`) 0 1.0)
        (`PrimitiveComponent.SetCustomPrimitiveDataFloat` (`self.BottomPillar`) 0 1.0)
        (else
          (`SceneComponent.SetHiddenInGame` _sm_doorpathblocker true false)
          (`PrimitiveComponent.SetCollisionEnabled` _sm_doorpathblocker_2 "NoCollision")
          (`PrimitiveComponent.SetCollisionEnabled` _box "NoCollision")
          (`LightComponent.SetIntensity` (`self.PointLight`) 0.0)
          (`PrimitiveComponent.SetCustomPrimitiveDataFloat` (`self.SM_DoorPathBlocker`) 0 1.0)
          (`PrimitiveComponent.SetCustomPrimitiveDataFloat` (`self.TopPillar`) 0 0.0)
          (`PrimitiveComponent.SetCustomPrimitiveDataFloat` (`self.MidPillar`) 0 0.0)
          (`PrimitiveComponent.SetCustomPrimitiveDataFloat` (`self.BottomPillar`) 0 0.0))))))