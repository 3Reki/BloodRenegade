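; BP_AriasMechanism is an interactable world mechanism that the blood character can activate.
; Overlapping its sphere registers it as the BP_BloodCharacter's current interactable, and leaving unregisters it.
; On Interact it calls StartActiveMechanisme, whose logic is not in this graph, then turns off the sphere's overlap events so it stops registering for interaction.
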(event `self.Interact`
  (`self.StartActiveMechanisme`)
  (set `PrimitiveComponent.bGenerateOverlapEvents` false (`self.Sphere`)))

(event `self.Sphere.OnComponentBeginOverlap`
  (params (OverlappedComponent :type "PrimitiveComponent Object Reference") (OtherActor :type "Actor Object Reference") (OtherComp :type "PrimitiveComponent Object Reference") (OtherBodyIndex :type Integer) (bFromSweep :type Boolean) (SweepResult :type "HitResult Structure (by ref)"))
  (bind _asbp_blood_character (cast `/Game/BP/BP_BloodCharacter` OtherActor))
  (`BloodCharacter.SetCurrentInteractable` _asbp_blood_character self))

(event `self.Sphere.OnComponentEndOverlap`
  (params (OverlappedComponent :type "PrimitiveComponent Object Reference") (OtherActor :type "Actor Object Reference") (OtherComp :type "PrimitiveComponent Object Reference") (OtherBodyIndex :type Integer))
  (bind _asbp_blood_character (cast `/Game/BP/BP_BloodCharacter` OtherActor))
  (`BloodCharacter.UnsetInteractable` _asbp_blood_character self))

(fn `UserConstructionScript`)