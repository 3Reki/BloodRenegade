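; BP_TriggerObjectif is a one-shot box trigger that uses its objective component when the player pawn walks into it.
; The first overlap by any actor sets IsConsumed, but only the player pawn activates BPObjectiveAC and records the trigger as a consumable through the GameInstance, without flushing the save.
; On BeginPlay, Load restores IsConsumed from existing save data, keyed by the actor's object name.
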(event `self.ReceiveBeginPlay`
  (`self.Load`))

(event `self.Box.OnComponentBeginOverlap`
  (params (OverlappedComponent :type "PrimitiveComponent Object Reference") (OtherActor :type "Actor Object Reference") (OtherComp :type "PrimitiveComponent Object Reference") (OtherBodyIndex :type Integer) (bFromSweep :type Boolean) (SweepResult :type "HitResult Structure (by ref)"))
  (if (not (`self.IsConsumed`))
    (set `self.IsConsumed` true)
    (if (== OtherActor (`GameplayStatics.GetPlayerPawn` 0))
      (`/Game/BP/Interactable/BP_Objective_AC.Use` (`self.BP_Objective_AC`))
      (message `/Game/BP/SaveSystem/BPI_Saver.SaveConsumable` (`GameplayStatics.GetGameInstance`) (`KismetSystemLibrary.GetObjectName` self) false))))

(fn `Load`
  (bind (_savegamedata _saveexists) (message `/Game/BP/SaveSystem/BPI_Saver.GetSaveData` (`GameplayStatics.GetGameInstance`)))
  (if _saveexists
    (set `self.IsConsumed` (`BlueprintSetLibrary.Set_Contains` (`/Game/BP/SaveSystem/BP_SaveGame.Consumables` _savegamedata) (`KismetSystemLibrary.GetObjectName` self)))
    (return)
    (else
      (return))))

(fn `UserConstructionScript`)