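; Player character Blueprint for the vampire, handling its presentation and save state.
; Effect events drive timelines into material parameter collections, primitive data, Niagara and camera for vampiric vision, Nightmare Form, bites, hook dissolve, light burning, hits and death.
; It also restores saved transform and blood gauge, creates subtitles, applies brightness and plays the ending sequence.
; Most illumination-probe detection and debug code is disabled or unwired.
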(event Custom|UpdateLightStatus
  ;[1 1 0.25] Illumination Detection Example Framework
  ;;[0 0.9489 1] Set Debug Indicator Color based on Overall Player Illumination
  (if (Variables|Default|GetDrawDebugBox)
    (Rendering|Debug|DrawDebugBox (+ (Transformation|GetActorLocation) "0, 0,100.000000") "1.000000,1.000000,1.000000" (Math|Color|Lerp(LinearColor) :B (Variables|Default|GetPlayer%20Illum%20Color) :Alpha (Variables|Default|GetPlayer%20Illumination)) "0, 0, 0" 0.0 1e+01)
    (Rendering|Debug|DrawDebugString (+ (Transformation|GetActorLocation) "-110.000000,0.000000,150.000000") (Utilities|String|Append "Overall player illumination = " (Utilities|String|ToString(Float) (Variables|Default|GetPlayer%20Illumination))) 0 (Math|Color|Lerp(LinearColor) :B (Variables|Default|GetPlayer%20Illum%20Color) :Alpha (Variables|Default|GetPlayer%20Illumination)))))

(event Custom|ResetCameraFocus
  (bind _returnvalue (Pawn|GetController))
  (bind _cameradezoom (Timeline|ResetStick PlayFromStart)
    (:Update
      (Pawn|SetControlRotation _returnvalue (Math|Rotator|Lerp(Rotator) (Pawn|GetControlRotation _returnvalue :!class /Script/Engine.Controller) (Transformation|GetActorRotation) _cameradezoom true)))))

(event Custom|AddWidgetSubtitle
  ;[1 1 1] Subtitles
  (bind _returnvalue (UserInterface|CreateWidget "/Game/BP/Widgets/WBP_Subtitles.WBP_Subtitles_C"))
  (bind _output_get (Variables|Default|SetSubtitles%20Widget _returnvalue))
  (Variables|/Game/BP/Widgets/WBP_Subtitles.WBP_Subtitles_C|SetTimerSubtitle _output_get (Variables|/Script/BloodRenegade.DialogueDataAsset|GetSubtitleTimer (Variables|Default|GetDADialogue)))
  (UserInterface|Viewport|AddtoViewport _output_get 0))

(event Custom|SetActiveProb
  (params (B :type Boolean))
  ;[0 1 0.25 1 24] DEBUG VIZ
  ;;[0 1 0.04559] ToggleDebugVis
  (if B
    (bind _outactors (Actor|GetAllActorsOfClass "/Game/IlluminationDetection/Blueprints/IlluminationVolumes/BP_IlluminationVolumeMaster.BP_IlluminationVolumeMaster_C"))
    (for _array_element _outactors
      (Default|UpdateBoundsVisibility _array_element true))
    (for _array_element_2 (Variables|Default|GetLightProbes)
      (Variables|/Game/IlluminationDetection/Blueprints/IlluminationComponents/BP_IlluminationProbe.BP_IlluminationProbe_C|SetDebugTraceLine _array_element_2 "None")
      (bind _output_get (Variables|/Game/IlluminationDetection/Blueprints/IlluminationComponents/BP_IlluminationProbe.BP_IlluminationProbe_C|SetDebugProbeStats _array_element_2 false))
      (Variables|Default|SetDrawDebugBox _output_get))
    (else
      (bind _outactors_2 (Actor|GetAllActorsOfClass "/Game/IlluminationDetection/Blueprints/IlluminationVolumes/BP_IlluminationVolumeMaster.BP_IlluminationVolumeMaster_C"))
      (for _array_element_3 _outactors_2
        (Default|UpdateBoundsVisibility _array_element_3 true))
      (for _array_element_4 (Variables|Default|GetLightProbes)
        (Variables|/Game/IlluminationDetection/Blueprints/IlluminationComponents/BP_IlluminationProbe.BP_IlluminationProbe_C|SetDebugTraceLine _array_element_4 "None")
        (bind _output_get_2 (Variables|/Game/IlluminationDetection/Blueprints/IlluminationComponents/BP_IlluminationProbe.BP_IlluminationProbe_C|SetDebugProbeStats _array_element_4 false))
        (Variables|Default|SetDrawDebugBox _output_get_2)))))

(event Custom|IsRagdoll
  ;[1 1 1] Death Ragdoll
  ;;[1 1 1] Ragdoll
  (Collision|SetCollisionProfileName (Variables|Character|GetMesh) "Ragdoll" true :!class /Script/Engine.PrimitiveComponent)
  (Physics|SetSimulatePhysics (Variables|Character|GetMesh) true)
  (Physics|SetEnableGravity (Variables|Character|GetMesh) true))

(event EventEffectDash
  ;[1 1 1] Mobilty - Hook / Vault / Ledge Jump
  (Components|Activation|Activate (Variables|Default|GetDashEffect) true))

(event EventTick
  (params (DeltaSeconds :type Float%20%28single-precision%29))
  ;[1 1 0.25] Illumination Detection Example Framework
  ;;[1 0.1381 0] Evaluate overall player illumination on tick
  (bind _overallillumination (CallFunction|CheckOverallIllumination (Variables|Default|GetLightProbes)))
  (Variables|Default|SetPlayer%20Illumination _overallillumination)
  (bind _linearcolor (CallFunction|CheckOverallColor (Variables|Default|GetLightProbes)))
  (Variables|Default|SetPlayer%20Illum%20Color _linearcolor)
  (if (<= (Variables|Default|GetPlayer%20Illumination) (Variables|Default|GetMinimumEmissiveLight))
    (bind _emissivetrack (Timeline|EmissiveFade Play)
      (:Update
        (Rendering|Material|SetScalarParameterValue "/Game/GameArt/MasterMaterial/MaterialParameterCollection/CharMPC/MPC_Char.MPC_Char" "GlowInTheDark" _emissivetrack :!class /Script/Engine.KismetMaterialLibrary)))
    (else
      (Timeline|EmissiveFade Reverse))))

(event EventEffectAfterHook
  ;[1 1 1] Mobilty - Hook / Vault / Ledge Jump
  (Variables|Default|SetIsHiddenDash false)
  (Components|Activation|Activate (Variables|Default|GetNS_HookLanding) true)
  (bind _dissolve (Timeline|DissolveTimeline Reverse)
    (:Update
      (Rendering|Material|SetCustomPrimitiveDataFloat (Variables|Character|GetMesh) 0 _dissolve))
    (:Finished
      (Rendering|SetVisibility (Variables|Character|GetMesh) (not (Variables|Default|GetIsHiddenDash)) false)
      (bind _glow (Timeline|ClothGlowDown PlayFromStart)
        (:Update
          (Rendering|Material|SetCustomPrimitiveDataFloat (Variables|Character|GetMesh) 1 _glow))))))

(event EventEffectEndNightmareForm
  (bind _nightformwingfilamentcombine (Variables|Default|GetNightformWIngFilamentCombine))
  ;[1 1 1] Nightmare Form
  (Components|Activation|Deactivate (Variables|Default|GetNightmareAreaVFX))
  (bind _fadein (Timeline|WingFadeOut ReverseFromEnd)
    (:Update
      (Rendering|Material|SetCustomPrimitiveDataFloat (Variables|Default|GetNightmareFormWings) 0 _fadein)
      (Rendering|Material|SetCustomPrimitiveDataFloat _nightformwingfilamentcombine 0 _fadein)
      (Rendering|Material|SetCustomPrimitiveDataFloat _nightformwingfilamentcombine 1 (* _fadein 25.0))
      (Rendering|Material|SetCustomPrimitiveDataFloat _nightformwingfilamentcombine 2 (* _fadein 2e+01))
      (bind _fadeout (Timeline|FadeOutArea Play)
        (:Update
          (Rendering|Material|SetScalarParameterValue (Variables|Default|GetMaterialCollection) (Utilities|Name|MakeLiteralName "DebugNightmareZone") _fadeout :!class /Script/Engine.KismetMaterialLibrary))))))

(event EventLoadPlayerSave
  (bind (_savegamedata _saveexists) (Class|BPISaver|GetSaveData(Message) (Game|GetGameInstance)))
  (if _saveexists
    (Class|BloodCharacter|SetBloodGauge (.BloodGaugeFill (Utilities|Struct|BreakS_PlayerSaveData (Variables|/Game/BP/SaveSystem/BP_SaveGame.BP_SaveGame_C|GetPlayerSave _savegamedata))))
    (Transformation|SetActorTransform (.Transform (Utilities|Struct|BreakS_PlayerSaveData (Variables|/Game/BP/SaveSystem/BP_SaveGame.BP_SaveGame_C|GetPlayerSave _savegamedata))) false true)
    (Pawn|SetControlRotation (Game|GetPlayerController 0) (.Rotation (Math|Transform|BreakTransform (.Transform (Utilities|Struct|BreakS_PlayerSaveData (Variables|/Game/BP/SaveSystem/BP_SaveGame.BP_SaveGame_C|GetPlayerSave _savegamedata))))))))

(event EventUpdateChangeForm
  (params (f :type Float%20%28single-precision%29))
  ;[1 1 1] VFX
  (Rendering|Material|SetScalarParameterValue (Variables|Default|GetMaterialCollection) (Utilities|Name|MakeLiteralName "HairColorSwapScalar") f :!class /Script/Engine.KismetMaterialLibrary))

(event EventStartVampiricVisionEffect
  (bind (_direction _fadesphere _desatcurve) (Timeline|FadeVampiricSense Play)
    (:Update
      (bind _returnvalue (Class|BloodCharacter|GetVampiricSphereMesh))
      (Rendering|Material|SetCustomPrimitiveDataFloat _returnvalue 0 _fadesphere)
      (if (not (Variables|/Script/BloodRenegade.BloodPlayerState|GetIsInNightmareForm (Utilities|ResolveSoftReference (Variables|Default|GetCurrentPlayerState))))
        (Rendering|Material|SetScalarParameterValue (Variables|Default|GetMaterialCollection) (Utilities|Name|MakeLiteralName "VampiricSenseDesat") _desatcurve :!class /Script/Engine.KismetMaterialLibrary)))))

(event EventCancelVampiricVisionEffect
  (bind (_direction _fadesphere _desatcurve) (Timeline|FadeVampiricSense Reverse)
    (:Update
      (bind _returnvalue (Class|BloodCharacter|GetVampiricSphereMesh))
      (Rendering|Material|SetCustomPrimitiveDataFloat _returnvalue 0 _fadesphere)
      (if (not (Variables|/Script/BloodRenegade.BloodPlayerState|GetIsInNightmareForm (Utilities|ResolveSoftReference (Variables|Default|GetCurrentPlayerState))))
        (Rendering|Material|SetScalarParameterValue (Variables|Default|GetMaterialCollection) (Utilities|Name|MakeLiteralName "VampiricSenseDesat") _desatcurve :!class /Script/Engine.KismetMaterialLibrary)))))

(event EventSetBlendMask
  (params (b :type Boolean))
  (if b
    (bind _lerp (Timeline|TimelineMaskBlend Play)
      (:Update
        (Variables|Default|SetBlendMaskPercent _lerp)))
    (else
      (Timeline|TimelineMaskBlend Reverse))))

(event EventEffectScanVampiricVision
  (bind _fadevampiricsense (Timeline|Timeline_0 PlayFromStart)
    (:Update
      (Rendering|Material|SetScalarParameterValue (Variables|Default|GetMaterialCollection) (Utilities|Name|MakeLiteralName "ScanTime") _fadevampiricsense :!class /Script/Engine.KismetMaterialLibrary))))

(event EventEffectTargetBlindLock
  (params (Position :type Vector :default "0, 0, 0"))
  (bind _returnvalue (Utilities|Name|MakeLiteralName "r_wrist"))
  (bind _mesh (Variables|Character|GetMesh))
  (bind _returnvalue_2 (Niagara|SpawnSystemAttached "/Game/GameArt/VFX/NiagaraSystem/Blindness/NS_BlindTrailTarget.NS_BlindTrailTarget" _mesh _returnvalue (Transformation|GetSocketLocation _mesh (Class|SkinnedMeshComponent|GetSocketBoneName _mesh _returnvalue)) "0, 0, 0" "KeepWorldPosition" true false))
  (Class|NiagaraComponent|SetVariablePosition _returnvalue_2 "CharStart" (Math|Vector|GetForwardVector _mesh))
  (Niagara|SetNiagaraVariable(Vector3) _returnvalue_2 "Target" Position)
  (Components|Activation|SetActive _returnvalue_2 true false))

(event EventInLightEffect
  (params (InLight :type Boolean))
  ;[1 1 1] VFX
  (if InLight
    (bind _burningcurve (Timeline|BurningDamage Play)
      (:Update
        (Rendering|Material|SetScalarParameterValue (Variables|Default|GetMaterialCollection) (Utilities|Name|MakeLiteralName "BurningIntensity") _burningcurve :!class /Script/Engine.KismetMaterialLibrary)))
    (else
      (Timeline|BurningDamage Reverse))))

(event EventFinisherBite
  (bind _returnvalue (Game|GetPlayerController 0))
  ;[1 0.5752 0.2776] Finisher Long Bite
  (Utilities|FlowControl|FlipFlop
    (:A
      (Game|Player|SetViewTargetwithBlend _returnvalue (Variables|/Script/Engine.ChildActorComponent|GetChildActor (Variables|Default|GetChildActor)) 0.2 "VTBlend_EaseInOut" 1.0 false)
      (Sequencer|Player|Play (Variables|/Script/ActorSequence.ActorSequenceComponent|GetSequencePlayer (Variables|Default|GetActorSequence)) :!class /Script/MovieScene.MovieSceneSequencePlayer))
    (:B
      (Game|Player|SetViewTargetwithBlend _returnvalue self 0.5 "VTBlend_EaseInOut" 1.0 false))))

(event EventEffectDeath
  (bind _followcamera (Variables|Default|GetFollowCamera))
  (bind _relativerotation (Variables|/Script/Engine.SceneComponent|GetRelativeRotation _followcamera))
  ;[1 1 1] Death Ragdoll
  (bind (_direction _cameradezoom _camerarotate) (Timeline|PlayerDeathCamera PlayFromStart)
    (:Update
      (Transformation|SetRelativeLocationAndRotation _followcamera (Math|Vector|Lerp(Vector) (Variables|/Script/Engine.SceneComponent|GetRelativeLocation _followcamera) "-208.000000,0.000000,156.000000" _cameradezoom) (Math|Rotator|Lerp(Rotator) (Variables|/Script/Engine.SceneComponent|GetRelativeRotation _followcamera) (Math|Rotator|MakeRotator (.roll _relativerotation) -37.0 (.yaw _relativerotation)) _camerarotate) false false))))

(event EventTakeHitEffect
  (params (b :type Boolean))
  ;[1 1 1] VFX
  ;;[1 1 1] Take hit = Blood screen
  (if b
    (bind _lerp (Timeline|Timeline PlayFromStart)
      (:Update
        (Rendering|Material|SetScalarParameterValue (Variables|Default|GetMaterialCollection) (Utilities|Name|MakeLiteralName "Health") _lerp :!class /Script/Engine.KismetMaterialLibrary)))
    (else
      (Timeline|Timeline ReverseFromEnd))))

(event EventSetBiteEffects
  (params (b :type Boolean))
  ;[1 1 1] VFX
  ;;[0.3229 0.3229 0.3229] Bite FX setup
  ;;;[1 1 1] Blood on char
  (if b
    (Components|Timeline|SetPlayRate (Variables|Default|GetLerpBloodEffect) 1.0)
    (bind (_direction _lerppp _lerpzoom) (Timeline|LerpBloodEffect Play)
      (:Update
        (Camera|SetFieldOfView (Variables|Default|GetFollowCamera) (Math|Float|Lerp 9e+01 6e+01 _lerpzoom))
        (Rendering|Material|SetScalarParameterValue "/Game/GameArt/MasterMaterial/MaterialParameterCollection/CharMPC/MPC_Char.MPC_Char" "BiteEffect" (Math|Float|Lerp -0.1 0.6 _lerppp) :!class /Script/Engine.KismetMaterialLibrary)))
    (else
      (bind (_direction_2 _bloodinessamount _faceexpression) (Timeline|isBloodyOverTime PlayFromStart)
        (:Update
          (Rendering|Material|SetScalarParameterValue "/Game/GameArt/MasterMaterial/MaterialParameterCollection/CharMPC/MPC_Char.MPC_Char" "BloodyLerp" _bloodinessamount :!class /Script/Engine.KismetMaterialLibrary)
          (Components|SkeletalMesh|SetMorphTarget (Variables|Character|GetMesh) "Rage" _faceexpression true)
          (Components|Timeline|SetPlayRate (Variables|Default|GetLerpBloodEffect) 2.0)
          (Timeline|LerpBloodEffect Reverse))))))

(event EventKillEffects
  ;[1 1 1] VFX
  ;;[0.3229 0.3229 0.3229] Bite FX setup
)

(event EventBloodSplash
  ;[1 1 1] VFX
  ;;[0.3229 0.3229 0.3229] Bite FX setup
  ;;;[1 1 1] Blood on char
  (Components|Activation|Activate (Variables|Default|GetBiteBloodSplash) true))

(event EventStartEndGame
  (Variables|Default|SetCustomTimeDilation 1.0)
  (Utilities|Time|SetGlobalTimeDilation 1.0)
  (bind _outactor (Sequencer|Player|CreateLevelSequencePlayer "/Game/GameArt/Sequences/ENDING_EYES.ENDING_EYES"))
  (Sequencer|Player|Play (Variables|/Script/LevelSequence.LevelSequenceActor|GetSequencePlayer _outactor) :!class /Script/MovieScene.MovieSceneSequencePlayer)
  (Utilities|FlowControl|Delay 12.1) ; Timer Cutscene End (Lulu)
  (Game|OpenLevel(byName) "L_StartProto"))

(event EventBeginPlay
  (bind _returnvalue (Class|BloodGameUserSettings|GetBloodGameUserSettings))
  (CallFunction|ChangeBrightness (Variables|/Script/BloodRenegade.BloodGameUserSettings|GetBrightness _returnvalue))
  ;[1 1 1] Subtitles
  (Variables|Default|SetVisiblePoint (Variables|Default|GetVisibleP))
  (CallFunction|AddWidgetSubtitle)
  (Rendering|Material|SetScalarParameterValue (Variables|Default|GetMaterialCollection) (Utilities|Name|MakeLiteralName "HairColorSwapScalar") 0.0 :!class /Script/Engine.KismetMaterialLibrary))

(event EventEffectStartNightmareForm
  ;[1 1 1] Nightmare Form
  (Components|Activation|Activate (Variables|Default|GetNightmareFormBurstIn) true)
  (Rendering|SetVisibility (Variables|Default|GetNightformWIngFilamentCombine) true false)
  (Rendering|SetVisibility (Variables|Default|GetNightmareFormWings) true false)
  (Rendering|Material|SetScalarParameterValue (Variables|Default|GetMaterialCollectionNF) (Utilities|Name|MakeLiteralName "WingsFade") 1.0 :!class /Script/Engine.KismetMaterialLibrary)
  (Rendering|Material|SetScalarParameterValue (Variables|Default|GetMaterialCollection) (Utilities|Name|MakeLiteralName "HairColorSwapScalar") 1.0 :!class /Script/Engine.KismetMaterialLibrary))

(event EventEffectBeforeHook
  ;[1 1 1] Mobilty - Hook / Vault / Ledge Jump
  (Variables|Default|SetIsHiddenDash true)
  (Components|Activation|Activate (Variables|Default|GetDashEffect) true)
  (Rendering|Material|SetCustomPrimitiveDataFloat (Variables|Character|GetMesh) 1 0.4)
  (bind _dissolve (Timeline|DissolveTimeline Play)
    (:Update
      (Rendering|Material|SetCustomPrimitiveDataFloat (Variables|Character|GetMesh) 0 _dissolve))
    (:Finished
      (Rendering|SetVisibility (Variables|Character|GetMesh) (not (Variables|Default|GetIsHiddenDash)) false)
      (bind _glow (Timeline|ClothGlowDown PlayFromStart)
        (:Update
          (Rendering|Material|SetCustomPrimitiveDataFloat (Variables|Character|GetMesh) 1 _glow))))))

(event Input|KeyboardEvents|DebugKeyJ
  (params (Key :type Key%20Structure :default "None") (ActionValue :type Input%20Action%20Value%20Structure))
  (:Pressed
    (Class|BiteSystem|ToggleShowBiteRange (Variables|Default|GetBiteSystem))))

(event Input|KeyboardEvents|L
  (params (Key :type Key%20Structure :default "None"))
  ;[0 1 0.25 1 24] DEBUG VIZ
  ;;[0 1 0.04559] Test turning off light volumes
  (:Pressed
    (Utilities|FlowControl|FlipFlop
      (:A
        (bind _outactors (Actor|GetAllActorsOfClass "/Game/IlluminationDetection/Blueprints/IlluminationVolumes/BP_IlluminationVolumeMaster.BP_IlluminationVolumeMaster_C"))
        (for _array_element _outactors
          (Default|SetLightStatus _array_element "NewEnumerator1")))
      (:B
        (bind _outactors_2 (Actor|GetAllActorsOfClass "/Game/IlluminationDetection/Blueprints/IlluminationVolumes/BP_IlluminationVolumeMaster.BP_IlluminationVolumeMaster_C"))
        (for _array_element_2 _outactors_2
          (Default|SetLightStatus _array_element_2 "NewEnumerator0"))))))

(fn ConstructionScript
  ;[1 1 1] ActivateSeethrough
  (Rendering|Material|SetScalarParameterValue "/Game/GameArt/MasterMaterial/MaterialParameterCollection/CharMPC/MPC_Char.MPC_Char" "SeeThrough" 1.0 :!class /Script/Engine.KismetMaterialLibrary))

(fn SetPointLightStatusExampleFunction
  (params (PointLightReference :type Object%20Object%20Reference) (Status :type EN_LightStatus%20Enum :default "NewEnumerator0"))
  (bind _outactors (Actor|GetAllActorsOfClass "/Game/IlluminationDetection/Blueprints/IlluminationVolumes/BP_IlluminationVolumeMaster.BP_IlluminationVolumeMaster_C"))
  (bind _array_element (Utilities|Array|ForEachLoopwithBreak _outactors :!label _label)
    (:LoopBody
      (if (== (Variables|/Game/IlluminationDetection/Blueprints/IlluminationVolumes/BP_IlluminationVolumeMaster.BP_IlluminationVolumeMaster_C|GetPL_Ref _array_element) PointLightReference)
        (Default|SetLightStatus _array_element Status)
        (goto _label Break)))
    (:Completed
      (return))))

(fn SetSpotLightStatusExampleFunction
  (params (SpotlightReference :type Object%20Object%20Reference) (Status :type EN_LightStatus%20Enum :default "NewEnumerator0"))
  (bind _outactors (Actor|GetAllActorsOfClass "/Game/IlluminationDetection/Blueprints/IlluminationVolumes/BP_IlluminationVolumeMaster.BP_IlluminationVolumeMaster_C"))
  (bind _array_element (Utilities|Array|ForEachLoopwithBreak _outactors :!label _label)
    (:LoopBody
      (if (== (Variables|/Game/IlluminationDetection/Blueprints/IlluminationVolumes/BP_IlluminationVolumeMaster.BP_IlluminationVolumeMaster_C|GetSL_Ref _array_element) SpotlightReference)
        (Default|SetLightStatus _array_element Status)
        (goto _label Break)))
    (:Completed
      (return))))

(fn GetPlayerSave
  (return (Utilities|Struct|MakeS_PlayerSaveData (Transformation|GetActorTransform) (Variables|/Script/BloodRenegade.BloodPlayerState|GetCurrentBloodGauge (Utilities|ResolveSoftReference (Variables|Default|GetCurrentPlayerState))))))

(fn AddSubtitle
  (params (NewText :type Text))
  (bind _subtitles_widget (Variables|Default|GetSubtitles%20Widget))
  (Utilities|IsValid _subtitles_widget
    (:Is%20Valid
      (Default|AddSubtitles _subtitles_widget NewText))))

(fn ChangeBrightness
  (params (Brightness :type Float%20%28double-precision%29))
  (bind _postprocessvolume (Variables|Default|GetPostProcessVolume))
  (bind _output_get (Variables|Default|SetBrightness Brightness))
  (bind _structout (Utilities|Struct|SetmembersinPostProcessSettings (Variables|/Script/Engine.PostProcessComponent|GetSettings _postprocessvolume) (Math|Vector4|MakeVector4 (Math|Float|Lerp 1.0 3.0 _output_get) (Math|Float|Lerp 1.0 3.0 _output_get) (Math|Float|Lerp 1.0 3.0 _output_get) (Math|Float|Lerp 1.0 3.0 _output_get))))
  (Variables|/Script/Engine.PostProcessComponent|SetSettings _postprocessvolume _structout))