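; BP_BloodController is a player controller that restores the player's saved input settings through Enhanced Input.
; On BeginPlay it re-applies remapped keys from BloodGameUserSettings to slot 1 of each mapping.
; A one-shot control-mappings-rebuilt callback then unbinds itself and applies saved mouse and controller X/Y sensitivities.
; An editor-only debug key on M calls the game pause function.
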(event Custom|LoadInputSettings
  (EventDispatchers|UnbindEventfromControlMappingsRebuiltDelegate (PlayerController|LocalPlayerSubsystems|GetEnhancedInputLocalPlayerSubsystem self) (delegate Custom|LoadInputSettings))
  (bind _returnvalue (Class|BloodGameUserSettings|GetBloodGameUserSettings))
  (Class|BloodController|UpdateMouseSensitivityX (Class|BloodGameUserSettings|GetMouseXSensitivity _returnvalue))
  (Class|BloodController|UpdateMouseSensitivityY (Class|BloodGameUserSettings|GetMouseYSensitivity _returnvalue))
  (Class|BloodController|UpdateControllerSensitivityX (Class|BloodGameUserSettings|GetControllerXSensitivity _returnvalue))
  (Class|BloodController|UpdateControllerSensitivityY (Class|BloodGameUserSettings|GetControllerYSensitivity _returnvalue)))

(event EventBeginPlay
  (EventDispatchers|BindEventtoControlMappingsRebuiltDelegate (PlayerController|LocalPlayerSubsystems|GetEnhancedInputLocalPlayerSubsystem self) (delegate Custom|LoadInputSettings))
  (bind _returnvalue (Class|BloodGameUserSettings|GetBloodGameUserSettings))
  (bind _keys (Utilities|Map|Keys (Variables|/Script/BloodRenegade.BloodGameUserSettings|GetMappedKeyInfos _returnvalue)))
  (for _array_element _keys
    (Class|EnhancedInputSubsystemInterface|AddPlayerMappedKeyinSlot (PlayerController|LocalPlayerSubsystems|GetEnhancedInputLocalPlayerSubsystem self) _array_element (.Value (Utilities|Map|Find (Variables|/Script/BloodRenegade.BloodGameUserSettings|GetMappedKeyInfos _returnvalue) _array_element)) (Utilities|Struct|MakePlayerMappableKeySlot 1) "(bIgnoreAllPressedKeysUntilRelease=True,bForceImmediately=False)")))

(event Input|KeyboardEvents|DebugKeyM
  (params (Key :type Key%20Structure :default "None") (ActionValue :type Input%20Action%20Value%20Structure))
  (:Pressed
    (Class|BloodBlueprintUtils|WithEditor
      (:True
        (Class|BloodController|SetGamePause)))))

(fn ConstructionScript)