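; Game instance for the Blood game that owns checkpoint-style save data per level and applies user settings on startup.
; Saves and loads a BP_SaveGame in slots named by save name plus current level, writing asynchronously.
; Save events update player, consumable, soldier, actor and objective data in memory, flushing to disk only when requested.
; In editor, startup wipes all slots and picks MainLevel or GymRoom from the map name.
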(event `self.ReceiveInit`
  (`BloodBlueprintUtils.WithEditor`
    (:`True`
      (`self.ResetSaveData`)
      (bind _returnvalue (`GameplayStatics.GetCurrentLevelName` true))
      (set `self.CurrentLevel` (`KismetMathLibrary.SelectString` "MainLevel" "GymRoom" (`KismetStringLibrary.EqualEqual_StrStr` _returnvalue "L_BloodMap"))))
    (:`False`
      _))
  (bind _returnvalue_2 (`BloodGameUserSettings.GetBloodGameUserSettings`))
  (`BloodGameUserSettings.ApplyBloodSettings` _returnvalue_2))

(event `self.SaveGameData`
  (`AsyncActionHandleSaveGame.AsyncSaveGameToSlot` (`self.SaveGame`) (`KismetStringLibrary.Concat_StrStr` (`self.SaveSlotName`) "_" (`self.CurrentLevel`))
    (:`Completed`
      (`KismetSystemLibrary.LogString` "Game Saved" false)
      (`KismetSystemLibrary.PrintString` "Saved Game !"))))

(event `self.LoadGameData`
  (bind _returnvalue (`KismetStringLibrary.Concat_StrStr` (`self.SaveSlotName`) "_" (`self.CurrentLevel`)))
  (bind _returnvalue_2 (`GameplayStatics.DoesSaveGameExist` _returnvalue))
  (if _returnvalue_2
    (bind _returnvalue_3 (`GameplayStatics.LoadGameFromSlot` _returnvalue))
    (set `self.SaveGame` (cast `/Game/BP/SaveSystem/BP_SaveGame` _returnvalue_3 :!pure true))
    (set `self.SaveExists` true)
    (else
      (bind _returnvalue_4 (`GameplayStatics.CreateSaveGameObject` "/Game/BP/SaveSystem/BP_SaveGame.BP_SaveGame_C"))
      (set `self.SaveGame` _returnvalue_4)
      (set `self.SaveExists` false))))

(event `self.ResetSaveData`
  (`GameplayStatics.DeleteGameInSlot` (`KismetStringLibrary.Concat_StrStr` (`self.SaveSlotName`) "_MainLevel"))
  (`GameplayStatics.DeleteGameInSlot` (`KismetStringLibrary.Concat_StrStr` (`self.SaveSlotName`) "_GymRoom"))
  (`GameplayStatics.DeleteGameInSlot` (`KismetStringLibrary.Concat_StrStr` (`self.SaveSlotName`) "_None"))
  (bind _returnvalue (`GameplayStatics.CreateSaveGameObject` "/Game/BP/SaveSystem/BP_SaveGame.BP_SaveGame_C"))
  (set `self.SaveGame` _returnvalue))

(event `/Game/BP/SaveSystem/BPI_Saver.SavePlayerData`
  (params (PlayerData :type "/Game/BP/SaveSystem/S_PlayerSaveData Structure") (FlushSave :type Boolean))
  (set `/Game/BP/SaveSystem/BP_SaveGame.PlayerSave` PlayerData (`self.SaveGame`))
  (`self.SaveIf` FlushSave))

(event `/Game/BP/SaveSystem/BPI_Saver.SaveConsumable`
  (params (CheckpointID :type String) (FlushSave :type Boolean))
  (`BlueprintSetLibrary.Set_Add` (`/Game/BP/SaveSystem/BP_SaveGame.Consumables` (`self.SaveGame`)) CheckpointID)
  (`self.SaveIf` FlushSave))

(event `/Game/BP/SaveSystem/BPI_Saver.SaveSoldier`
  (params (SoldierID :type String) (IsActiveAtBeginPlay :type Boolean) (FlushSave :type Boolean))
  (`BlueprintMapLibrary.Map_Add` (`/Game/BP/SaveSystem/BP_SaveGame.SoldierSaves` (`self.SaveGame`)) SoldierID IsActiveAtBeginPlay)
  (`self.SaveIf` FlushSave))

(event `/Game/BP/SaveSystem/BPI_Saver.SaveActor`
  (params (ActorID :type String) (ActorTransform :type "Transform Structure") (FlushSave :type Boolean))
  (`BlueprintMapLibrary.Map_Add` (`/Game/BP/SaveSystem/BP_SaveGame.Actors` (`self.SaveGame`)) ActorID ActorTransform)
  (`self.SaveIf` FlushSave))

(event `/Game/BP/SaveSystem/BPI_Saver.SaveObjective`
  (params (ObjectiveName :type String) (FlushSave :type Boolean))
  (set `/Game/BP/SaveSystem/BP_SaveGame.Objective` ObjectiveName (`self.SaveGame`))
  (`self.SaveIf` FlushSave))

(fn `DoesSaveExists`
  (params (LevelName :type String))
  (returns (Exists :type Boolean))
  (bind _returnvalue (`GameplayStatics.DoesSaveGameExist` (`KismetStringLibrary.Concat_StrStr` (`self.SaveSlotName`) "_" LevelName)))
  (return _returnvalue))

(fn `GetSaveData`
  (returns (SaveGameData :type "/Game/BP/SaveSystem/BP_SaveGame Object Reference") (SaveExists :type Boolean))
  (bind _savegame (`self.SaveGame`))
  (`/Engine/EditorBlueprintResources/StandardMacros.IsValid` (`self.SaveGame`)
    (:`Is Valid`
      (return _savegame (`self.SaveExists`)))
    (:`Is Not Valid`
      (return _savegame false))))