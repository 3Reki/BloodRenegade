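; Enemy soldier for a vampire stealth game, handling presentation and state changes for detection, laser fire, bites, stuns, shielding, death and revival.
; Events pair Implementation calls with physics, gun, UV lamp and Niagara changes, while a widget indicator faces the camera.
; Timelines drive shield fade, dust-and-blood dissolve and vampiric-vision highlighting through custom primitive data, stencil and material parameters.
; Death saves the soldier as inactive, and LoadSave restores that flag.
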(event `self.CapsuleComponent.OnComponentBeginOverlap`
  (params (OverlappedComponent :type "PrimitiveComponent Object Reference") (OtherActor :type "Actor Object Reference") (OtherComp :type "PrimitiveComponent Object Reference") (OtherBodyIndex :type Integer) (bFromSweep :type Boolean) (SweepResult :type "HitResult Structure (by ref)"))
  (`self.OnOverlapBegin` OverlappedComponent OtherActor OtherComp OtherBodyIndex bFromSweep SweepResult))

(event `self.ReceiveBeginPlay`
  (bind _widgetcomponent (`self.WidgetComponent`))
  (bind _aswbp_enemy_detection (cast `/Game/BP/Widgets/WBP_EnemyDetection` (`WidgetComponent.GetWidget` _widgetcomponent)))
  (set `self.As WBP Detection Suspicious` _aswbp_enemy_detection)
  (set `self.WidgetScale` (`SceneComponent.K2_GetComponentScale` _widgetcomponent))
  (if (not (`AIManagerSubsystem.IsDetectionIndicatorVisible` (subsystem `AIManagerSubsystem`)))
    (`self.SetDetectionIndicatorVisible` false))
  (`PrimitiveComponent.SetCustomDepthStencilValue` (`self.Mesh`) 0)
  ;[1 1 1] set event
  (`NiagaraComponent.SetNiagaraVariableObject` (`self.LaserVFX`) "User.BP_CallbackSoldier" self)
  (`WeaponComponent.SetMuzzlePoint` (`self.WeaponComponent`) (`self.MuzzlePoint`))
  (`PrimitiveComponent.SetScalarParameterForCustomPrimitiveData` (`self.Mesh`) "EmissiveColorLerp" 0.0)
  (`self.Aim Laser Effect`))

(event `self.CapsuleComponent.OnComponentEndOverlap`
  (params (OverlappedComponent :type "PrimitiveComponent Object Reference") (OtherActor :type "Actor Object Reference") (OtherComp :type "PrimitiveComponent Object Reference") (OtherBodyIndex :type Integer))
  (`self.OnOverlapEnd` OverlappedComponent OtherActor OtherComp OtherBodyIndex))

(event `self.LoadSave`
  (bind (_savegamedata _saveexists) (message `/Game/BP/SaveSystem/BPI_Saver.GetSaveData` (`GameplayStatics.GetGameInstance`)))
  (bind (_value _returnvalue) (`BlueprintMapLibrary.Map_Find` (`/Game/BP/SaveSystem/BP_SaveGame.SoldierSaves` _savegamedata) (`KismetSystemLibrary.GetObjectName` self)))
  (if (and _saveexists _returnvalue)
    (set `self.StartEnabled` _value)))

(event `Aim Laser Effect`
  (bind _soldierda (`self.SoldierDA`))
  (bind _laserpointer (`self.LaserPointer`))
  ;[1 1 1] Fire effect
  (`ActorComponent.Activate` _laserpointer false)
  (`NiagaraComponent.SetVariableFloat` _laserpointer "LaserLength" (`SoldierDataAsset.FireRange` _soldierda))
  (`NiagaraComponent.SetVariableLinearColor` _laserpointer "LaserColor" (`SoldierDataAsset.LaserColor` _soldierda)))

(event `self.ReceiveTick`
  (params (DeltaSeconds :type "Float (single-precision)"))
  (`/Engine/EditorBlueprintResources/StandardMacros.IsValid` (`self.As WBP Detection Suspicious`)
    (:`Is Valid`
      (`SceneComponent.K2_SetWorldRotation` (`self.WidgetComponent`) (`KismetMathLibrary.Conv_VectorToRotator` (* (`self.GetActorForwardVector` (`GameplayStatics.GetPlayerCameraManager` 0)) -1)) false false))))

(event `self.AimEffect`
  (params (Direction :type "Vector Structure"))
  ;[1 1 1] Fire effect
  (`ActorComponent.Activate` (`self.ChargingLaser`) true))

(event `self.Blind_Event`
  (params (t :type "Float (single-precision)"))
  ;[1 1 1] Fire effect
  (`ActorComponent.Activate` false :!enabledstate Disabled)
  (`KismetSystemLibrary.PrintString` "Inside" :!enabledstate Disabled))

(event `self.BeingBite`
  (params (f :type "Float (single-precision)"))
  (bind _sk_soldier_gun (`self.SK_Soldier_Gun`))
  ;[1 0.5297 0.18] BEING BITE
  (`self.SetIsBeingBitten` true)
  (`self.Stun_Implementation` f)
  (`self.ChangeOutline` 0.0)
  (`SceneComponent.K2_DetachFromComponent` _sk_soldier_gun "KeepWorld" "KeepWorld" "KeepWorld" true)
  (`PrimitiveComponent.SetSimulatePhysics` _sk_soldier_gun true)
  (`PrimitiveComponent.SetCollisionEnabled` (`self.CapsuleComponent`) "NoCollision")
  (`MotherWorldElements.SwitchOff` (cast `/Game/BP/WorldElements/BP_UVLAMP` (`ChildActorComponent.ChildActor` (`self.UVLamp`)) :!pure true)))

(event `self.FireEffect`
  (params (TargetPosition :type "Vector Structure") (Direction :type "Vector Structure"))
  ;[1 1 1] Fire effect
  ;;[1 1 1] Fire
  (`NiagaraComponent.SetVariableVec3` (`self.LaserVFX`) "TargetPos" TargetPosition)
  (`NiagaraComponent.SetVariableVec3` (`self.LaserVFX`) "LaserDirection" Direction)
  (`NiagaraComponent.SetVariableFloat` (`self.LaserVFX`) "LaserLength" (`KismetMathLibrary.VSize` Direction))
  (`ActorComponent.Activate` (`self.LaserVFX`) true)
  ;;[1 1 1] Activate Impact
  (`NiagaraFunctionLibrary.SpawnSystemAtLocation` "/Game/GameArt/VFX/NiagaraSystem/EnnemyLaser/NS_HitLaser.NS_HitLaser" TargetPosition))

(event `self.Stun`
  (params (f :type "Float (single-precision)"))
  (`self.SetIsBeingBitten` false)
  (`self.Stun_Implementation` f))

(event `self.ReceiveParticleData`
  (params (Data :type "Array of BasicParticleData Structure (by ref)") (NiagaraSystem :type "NiagaraSystem Object Reference") (SimulationPositionOffset :type "Vector Structure (by ref)"))
  ;[1 1 1] Fire effect
  ;;[1 1 1] Fire
)

(event `self.Die`
  ;[1 0.3338 0.4438] DEATH
  (bind _asbp_uvlamp (cast `/Game/BP/WorldElements/BP_UVLAMP` (`ChildActorComponent.ChildActor` (`self.UVLamp`)))
    (:`then`
      (`MotherWorldElements.SwitchOff` _asbp_uvlamp))
    (:`CastFailed`
      _))
  (`self.BeingBite` 4.0)
  (`self.Die_Implementation`)
  (`PrimitiveComponent.SetCustomDepthStencilValue` (`self.Mesh`) 0)
  (`PrimitiveComponent.SetMaterial` (`self.Mesh`) 2 null)
  (message `/Game/BP/SaveSystem/BPI_Saver.SaveSoldier` (`GameplayStatics.GetGameInstance`) (`KismetSystemLibrary.GetObjectName` self) false false)
  (`PrimitiveComponent.SetCollisionEnabled` (`self.Mesh`) "PhysicsOnly")
  (`SceneComponent.SetVisibility` (`self.LensFlare`) false true)
  (`SceneComponent.SetVisibility` (`self.CharaLight`) false true)
  (`SceneComponent.SetVisibility` (`self.PoliceHologram`) false true)
  (`SceneComponent.SetVisibility` (`self.EmissiveFakeLight`) false true)
  (`PrimitiveComponent.SetScalarParameterForCustomPrimitiveData` (`self.Mesh`) "EmissiveIntensityBoost" 0.0))

(event `self.Revive`
  (bind _sk_soldier_gun (`self.SK_Soldier_Gun`))
  (bind _mesh (`self.Mesh`))
  (bind _mesh_2 (`self.Mesh`))
  ;[0 0.5035 1] REVIVE
  (`self.Revive_Implementation`)
  (`MotherWorldElements.SwitchOn` (cast `/Game/BP/WorldElements/BP_UVLAMP` (`ChildActorComponent.ChildActor` (`self.UVLamp`)) :!pure true))
  (`PrimitiveComponent.SetMaterial` (`self.Mesh`) 2 null)
  (`PrimitiveComponent.SetSimulatePhysics` _sk_soldier_gun false)
  (`SceneComponent.K2_AttachToComponent` _sk_soldier_gun (`self.Mesh`) "l_wristSocket" "SnapToTarget" "SnapToTarget" "KeepWorld" true)
  (`PrimitiveComponent.SetCollisionEnabled` (`self.CapsuleComponent`) "QueryAndPhysics")
  (`PrimitiveComponent.SetSimulatePhysics` _mesh false)
  (`PrimitiveComponent.SetCollisionEnabled` _mesh "QueryOnly")
  (`PrimitiveComponent.SetCollisionProfileName` _mesh_2 "Custom" true)
  (`SceneComponent.K2_AttachToComponent` _mesh_2 (`self.CapsuleComponent`) "None" "KeepWorld" "KeepWorld" "KeepWorld" true)
  (`SceneComponent.K2_SetRelativeLocationAndRotation` (`self.Mesh`) (0.0 0.0 -85.0) (struct :`Yaw` -90.0) false true)
  (`SceneComponent.SetVisibility` (`self.LensFlare`) true true)
  (`SceneComponent.SetVisibility` (`self.CharaLight`) true true)
  (`SceneComponent.SetVisibility` (`self.PoliceHologram`) true true)
  (`SceneComponent.SetVisibility` (`self.EmissiveFakeLight`) true true)
  (`PrimitiveComponent.SetScalarParameterForCustomPrimitiveData` (`self.Mesh`) "EmissiveIntensityBoost" 1.0)
  (`ActorComponent.Activate` (`self.AIPerceptionStimuliSource`) false))

(event `self.ShieldEffect`
  (bind _sm_legshield_l (`self.SM_LegShield_l`))
  ;[1 1 1] Shield
  (if (`self.IsShielded`)
    (`SceneComponent.SetHiddenInGame` _sm_legshield_l false false)
    (`SceneComponent.SetHiddenInGame` (`self.SM_BustShield`) false false)
    (`SceneComponent.SetHiddenInGame` (`self.SM_LegShield_r`) false false)
    (`SceneComponent.SetHiddenInGame` (`self.SM_ThighShield_l`) false false)
    (`SceneComponent.SetHiddenInGame` (`self.SM_ThighShield_r`) false false)
    (`SceneComponent.SetHiddenInGame` (`self.SM_NeckShield`) false false)
    (`SceneComponent.SetHiddenInGame` (`self.SM_BeltShield`) false false)
    (`SceneComponent.SetHiddenInGame` (`self.SM_SpaulderShield_r`) false false)
    (`SceneComponent.SetHiddenInGame` (`self.SM_ArmShield_l`) false false)
    (`SceneComponent.SetHiddenInGame` (`self.SM_ArmShield_r`) false false)
    (`SceneComponent.SetHiddenInGame` (`self.SM_SpaulderShield_l`) false false)
    (`SceneComponent.SetHiddenInGame` (`self.SM_BackShield`) false false)
    (bind (_direction _fadeshield) (`Timeline|FadeShield` :!label _label)
      (:`Update`
        (`PrimitiveComponent.SetCustomPrimitiveDataFloat` _sm_legshield_l 0 _fadeshield)
        (`PrimitiveComponent.SetCustomPrimitiveDataFloat` (`self.SM_BustShield`) 0 _fadeshield)
        (`PrimitiveComponent.SetCustomPrimitiveDataFloat` (`self.SM_LegShield_r`) 0 _fadeshield)
        (`PrimitiveComponent.SetCustomPrimitiveDataFloat` (`self.SM_ThighShield_l`) 0 _fadeshield)
        (`PrimitiveComponent.SetCustomPrimitiveDataFloat` (`self.SM_ThighShield_r`) 0 _fadeshield)
        (`PrimitiveComponent.SetCustomPrimitiveDataFloat` (`self.SM_NeckShield`) 0 _fadeshield)
        (`PrimitiveComponent.SetCustomPrimitiveDataFloat` (`self.SM_BeltShield`) 0 _fadeshield)
        (`PrimitiveComponent.SetCustomPrimitiveDataFloat` (`self.SM_SpaulderShield_r`) 0 _fadeshield)
        (`PrimitiveComponent.SetCustomPrimitiveDataFloat` (`self.SM_ArmShield_l`) 0 _fadeshield)
        (`PrimitiveComponent.SetCustomPrimitiveDataFloat` (`self.SM_ArmShield_r`) 0 _fadeshield)
        (`PrimitiveComponent.SetCustomPrimitiveDataFloat` (`self.SM_SpaulderShield_l`) 0 _fadeshield)
        (`PrimitiveComponent.SetCustomPrimitiveDataFloat` (`self.SM_BackShield`) 0 _fadeshield)
        (`PrimitiveComponent.SetCustomPrimitiveDataFloat` (`self.Mesh`) 3 (* 10.0 _fadeshield)))
      (:`Finished`
        (switch `ETimelineDirection` _direction
          (:`Backward`
            (`SceneComponent.SetHiddenInGame` _sm_legshield_l true false)
            (`SceneComponent.SetHiddenInGame` (`self.SM_BustShield`) true false)
            (`SceneComponent.SetHiddenInGame` (`self.SM_LegShield_r`) true false)
            (`SceneComponent.SetHiddenInGame` (`self.SM_ThighShield_l`) true false)
            (`SceneComponent.SetHiddenInGame` (`self.SM_ThighShield_r`) true false)
            (`SceneComponent.SetHiddenInGame` (`self.SM_NeckShield`) true false)
            (`SceneComponent.SetHiddenInGame` (`self.SM_BeltShield`) true false)
            (`SceneComponent.SetHiddenInGame` (`self.SM_SpaulderShield_r`) true false)
            (`SceneComponent.SetHiddenInGame` (`self.SM_ArmShield_l`) true false)
            (`SceneComponent.SetHiddenInGame` (`self.SM_ArmShield_r`) true false)
            (`SceneComponent.SetHiddenInGame` (`self.SM_SpaulderShield_l`) true false)
            (`SceneComponent.SetHiddenInGame` (`self.SM_BackShield`) true false)))))
    (else
      (goto _label :!via `Reverse`))))

(event `self.BiteSound`
  (params (IsSilent :type Boolean) (PlayLongSound :type Boolean))
  (`self.BiteSound_Implementation` IsSilent PlayLongSound))

(event `self.BeingArialBite`
  (bind _fakevisioncone (`self.FakeVisionCone`))
  (`self.BeingArialBite_Implementation`)
  (if (`KismetSystemLibrary.IsValid` _fakevisioncone) :!label _label_2
    (`ActorComponent.K2_DestroyComponent` _fakevisioncone)
    (`MotherWorldElements.SwitchOff` (cast `/Game/BP/WorldElements/BP_UVLAMP` (`ChildActorComponent.ChildActor` (`self.UVLamp`)) :!pure true))))

(event `self.BeingAttacked`
  (`self.BeingAttacked_Implementation`)
  (goto _label_2))

(event `self.SetDetectionIndicatorVisible`
  (params (Visible :type Boolean))
  (`Widget.SetVisibility` (`self.As WBP Detection Suspicious`) (select `bool` Visible :`false` "Hidden" :`true` "Visible" :!type "ESlateVisibility Enum")))

(event `self.Stun_Event`
  (params (t :type "Float (single-precision)"))
  ;[1 1 1] Called from blood char
  (if (not (`self.IsBeingBitten`))
    (`NiagaraComponent.SetVariableFloat` (`self.StunEffect`) "Lifetime" t)
    (`ActorComponent.Activate` (`self.StunEffect`) true)
    (`KismetSystemLibrary.Delay` t)
    (`ActorComponent.Deactivate` (`self.StunEffect`))))

(event `self.StartVampiricVisible`
  (params (f :type "Float (single-precision)"))
  (bind _sk_soldier_gun (`self.SK_Soldier_Gun`))
  (bind _mesh (`self.Mesh`))
  (bind _mesh_2 (`self.Mesh`))
  ;[0.8286 0.5374 1] START VAMPIRIC VISIBLE
  (`TimelineComponent.SetPlayRate` (`self.TimelineVV`) (/ 1.0 f))
  (if (not (`self.VVActivated`))
    (`PrimitiveComponent.SetCustomDepthStencilValue` (`self.SK_Soldier_Gun`) 1)
    (`PrimitiveComponent.SetCustomDepthStencilValue` _mesh (+ (`PrimitiveComponent.CustomDepthStencilValue` _mesh) 1))
    (set `self.VVActivated` true)
    (bind (_direction _vvtrack) (`Timeline|TimelineVV` :!via `PlayFromStart`)
      (:`Update`
        (`KismetMaterialLibrary.SetScalarParameterValue` (`self.MPCSoldier`) "VampiricVisionFade" _vvtrack))
      (:`Finished`
        (`PrimitiveComponent.SetCustomDepthStencilValue` _sk_soldier_gun (+ (`PrimitiveComponent.CustomDepthStencilValue` _sk_soldier_gun) -1))
        (`PrimitiveComponent.SetCustomDepthStencilValue` _mesh_2 (+ (`PrimitiveComponent.CustomDepthStencilValue` _mesh_2) -1))
        (set `self.VVActivated` false)))))

(event `self.BeingDissolved`
  (bind _blood (`self.Blood`))
  (`NiagaraComponent.SetVariableFloat` (`self.NS_ToDust`) "DissolveAmount" 0.0)
  (`ActorComponent.Activate` (`self.NS_ToDust`) false)
  (`SceneComponent.SetVisibility` _blood true false)
  (bind _returnvalue (`DecalComponent.CreateDynamicMaterialInstance` _blood))
  (bind (_direction _disolve _groundblood) (`Timeline|Timeline` :!via `PlayFromStart`)
    (:`Update`
      ;[1 1 1] Destroy the soldier instant at the end of the dissolve
      (`PrimitiveComponent.SetCustomPrimitiveDataFloat` (`self.Mesh`) 0 _disolve)
      (`NiagaraComponent.SetVariableFloat` (`self.NS_ToDust`) "DissolveAmount" _disolve)
      (`MaterialInstanceDynamic.SetScalarParameterValue` _returnvalue "Dissolve" _groundblood)
      (`ActorComponent.Deactivate` (`self.AIPerceptionStimuliSource`)))
    (:`Finished`
      (`SceneComponent.SetHiddenInGame` (`self.Mesh`) true false)
      (bind (_direction_2 _dissolveoutblood) (`Timeline|FadeOutBlood`)
        (:`Update`
          (`MaterialInstanceDynamic.SetScalarParameterValue` _returnvalue "Dissolve" _dissolveoutblood))
        (:`Finished`
          (`SceneComponent.SetVisibility` (`self.Blood`) false false))))))

(event `GetRagdolled`
  ;[1 1 1] RagdollEvent
  (`PrimitiveComponent.SetCollisionProfileName` (`self.Mesh`) "Ragdoll" true)
  (`PrimitiveComponent.SetSimulatePhysics` (`self.Mesh`) true))

(event `self.SuspiciousEffect`
  ;[1 1 1] Visiere color change
  (`PrimitiveComponent.SetScalarParameterForCustomPrimitiveData` (`self.Mesh`) "EmissiveColorLerp" 1.0))

(event `self.NeutralEffect`
  ;[1 1 1] Visiere color change
  (`PrimitiveComponent.SetScalarParameterForCustomPrimitiveData` (`self.Mesh`) "EmissiveColorLerp" 0.0))

(fn `GetBlindOffset`
  (returns (ReturnValue :type "Float (single-precision)"))
  (return 60.0))

(fn `UserConstructionScript`
  (`PrimitiveComponent.SetCustomPrimitiveDataFloat` (`self.Mesh`) 4 (`KismetMathLibrary.RandomFloat`)))