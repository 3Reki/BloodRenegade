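; Skill indicator Blueprint that shows targeting visuals for the Blind and Decoy skills.
; Blind toggles a target indicator effect, while Decoy activates a teleport indicator, grows it with a Timeline and reveals a preview mesh using the decoy material.
; Hiding Decoy reverses the Timeline, whose updates then zero the indicator size and hide the mesh.
; A separate event tints the teleport indicator red when there is not enough space, black otherwise.
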(event `self.ReceiveBeginPlay`
  (for (_ _array_index) (`MeshComponent.GetMaterials` (`self.Mesh1`))
    (`PrimitiveComponent.SetMaterial` (`self.Mesh1`) _array_index "/Game/GameArt/VFX/Materials/M_Decoy.M_Decoy")))

(event `self.BlindEffect`
  (params (isShowing :type Boolean))
  (bind _targetindicator (`self.TargetIndicator`))
  ;[1 1 1] Blind
  (if isShowing
    (`ActorComponent.Activate` _targetindicator true)
    (else
      (`ActorComponent.Deactivate` _targetindicator))))

(event `self.DecoyEffect`
  (params (isShowing :type Boolean))
  (bind _teleportindicator (`self.TeleportIndicator`))
  ;[1 1 1] Decoy
  (if isShowing
    (`ActorComponent.Activate` _teleportindicator true)
    (bind (_direction _fadeinindicatortrack) (`Timeline|Timeline` :!label _label)
      (:`Update`
        (if isShowing
          (`NiagaraComponent.SetVariableFloat` _teleportindicator "IndicatorSize" _fadeinindicatortrack)
          (`NiagaraComponent.SetVariableLinearColor` _teleportindicator "TeleportColor" (`KismetMathLibrary.LinearColor_Black`))
          (`SceneComponent.SetVisibility` (`self.Mesh1`) true false)
          (else
            (`NiagaraComponent.SetVariableFloat` _teleportindicator "IndicatorSize" 0.0)
            (`NiagaraComponent.SetVariableLinearColor` _teleportindicator "TeleportColor" (`KismetMathLibrary.LinearColor_Black`))
            (`SceneComponent.SetVisibility` (`self.Mesh1`) false false)))))
    (else
      (goto _label :!via `Reverse`))))

(event `self.NotSpaceDecoyEffect`
  (params (haveEnoughPlace :type Boolean))
  (bind _teleportindicator (`self.TeleportIndicator`))
  ;[1 1 1] Decoy
  (if haveEnoughPlace
    (`NiagaraComponent.SetVariableLinearColor` _teleportindicator "TeleportColor" (`KismetMathLibrary.LinearColor_Black`))
    (else
      (`NiagaraComponent.SetVariableLinearColor` _teleportindicator "TeleportColor" (`KismetMathLibrary.LinearColor_Red`)))))

(fn `UserConstructionScript`)