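; Interactable generator switch that the player shuts off once, switching off its linked ListInteract actors until ResetInteraction restores them.
; Box overlap registers it as the player's current interactable, while SoundSphere drives the presence audio.
; Shutdown emits AI noise, plays feedback, and can trigger objective or dialogue components and offset an actor.
; The last generator also plays a sequence, kills snipers, stuns soldiers, then starts endgame or nightmare form depending on survivors.
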(event `self.ReceiveBeginPlay`
  ;[1 1 1] Faire bouger un truc - Esther
  (if (`self.ObjMove?`)
    (set `self.ObjMoveLocation` (`self.K2_GetActorLocation` (`self.ObjMove`))))
  (`PrimitiveComponent.SetCustomPrimitiveDataFloat` (`self.Cube`) 1 1.0)
  (if (< (`KismetMathLibrary.Vector_DistanceSquared` (`self.K2_GetActorLocation` (`GameplayStatics.GetPlayerCharacter` 0)) (`SceneComponent.K2_GetComponentLocation` (`self.Cube`))) (`KismetMathLibrary.Square` (`SphereComponent.SphereRadius` (`self.SoundSphere`))))
    (`AkGameObject.PostAkEvent` :`self` (`self.Ak`) :`AkEvent` "/Game/WwiseAudio/Events/Environment_Work_Unit/SFX_Generator_Presence.SFX_Generator_Presence")))

(event `self.Interact`
  (bind _asbp_blood_character (cast `/Game/BP/BP_BloodCharacter` (`GameplayStatics.GetPlayerPawn` 0) :!pure true))
  (if (`self.IsOn`)
    (set `self.IsOn` false)
    (`LightComponent.SetIntensity` (`self.PointLight`) 0.0)
    (`PrimitiveComponent.SetCustomPrimitiveDataFloat` (`self.Cube`) 1 0.0)
    (for _array_element (`self.ListInteract`)
      (`MotherWorldElements.SwitchOff` _array_element))
    (`self.MakeNoise` 1.0 (`GameplayStatics.GetPlayerPawn` 0) (`self.K2_GetActorLocation`) (`BloodCharacterDataAsset.InteractSoundRange` (`self.DA_BloodCharacter`)) "Instant")
    (`ActorComponent.Activate` (`self.NS_GeneratorDown`) true)
    (`AkGameObject.PostAkEvent` :`self` (`self.Ak`) :`AkEvent` "/Game/WwiseAudio/Events/Environment_Work_Unit/SFX_Generator_TurnOff.SFX_Generator_TurnOff")
    (set `PrimitiveComponent.bGenerateOverlapEvents` false (`self.Box1`))
    (if (and (`self.SetObjective`) (`KismetSystemLibrary.IsValid` (`self.ObjectiveComponent`)))
      (`/Game/BP/Interactable/BP_Objective_AC.Use` (`self.ObjectiveComponent`)))
    (if (and (`self.PlayDialogue`) (`KismetSystemLibrary.IsValid` (`self.DialogueComponent`)))
      (`/Game/BP/Interactable/BP_Dialogue_AC.Use` (`self.DialogueComponent`)))
    ;[1 1 1] Faire bouger un truc - Esther
    (if (`self.ObjMove?`)
      (`self.K2_SetActorLocation` (`self.ObjMove`) (+ (`self.ObjMoveLocation`) (`self.ObjMoveOffset`)) false false))
    (if (`self.IsLastGenerator`)
      (bind _outactor (`LevelSequencePlayer.CreateLevelSequencePlayer` (`self.Sequence`)))
      (`MovieSceneSequencePlayer.Play` (`LevelSequenceActor.SequencePlayer` _outactor))
      (`SceneComponent.SetVisibility` (`Character.Mesh` _asbp_blood_character) false false)
      (set `Actor.bCanBeDamaged` false _asbp_blood_character)
      (`BloodCharacter.SetActiveNightmareForm` _asbp_blood_character)
      (`HealthSystem.ResetHP` (`BloodCharacter.HealthSystem` _asbp_blood_character))
      (for _array_element_2 (`self.SniperToDie`)
        (if (not (`Soldier.IsDead` _array_element_2))
          (`IBitable.Die` _array_element_2)))
      (for _array_element_3 (`self.SoldiersToDie`)
        (`IBitable.Stun` _array_element_3 100000.0)
        (if (not (`Soldier.IsDead` _array_element_3))
          (bind _result (`/Engine/EditorBlueprintResources/StandardMacros.IncrementInt` (`self.CurrentEnemyCounter`)))))
      (`KismetSystemLibrary.Delay` 5.8)
      (`SceneComponent.SetVisibility` (`Character.Mesh` _asbp_blood_character) true false)
      (if (== (`self.CurrentEnemyCounter`) 0)
        (`BloodCharacter.StartEndGame` _asbp_blood_character)
        (else
          (`BloodCharacter.StartNightmareForm` _asbp_blood_character _result))))))

(event `ResetInteraction`
  (set `self.IsOn` true)
  (`LightComponent.SetIntensity` (`self.PointLight`) 1.0)
  (`PrimitiveComponent.SetCustomPrimitiveDataFloat` (`self.Cube`) 1 1.0)
  (for _array_element (`self.ListInteract`)
    (`MotherWorldElements.SwitchOn` _array_element))
  (set `PrimitiveComponent.bGenerateOverlapEvents` true (`self.Box1`)))

(event `self.Box1.OnComponentBeginOverlap`
  (params (OverlappedComponent :type "PrimitiveComponent Object Reference") (OtherActor :type "Actor Object Reference") (OtherComp :type "PrimitiveComponent Object Reference") (OtherBodyIndex :type Integer) (bFromSweep :type Boolean) (SweepResult :type "HitResult Structure (by ref)"))
  (bind _asbp_blood_character (cast `/Game/BP/BP_BloodCharacter` OtherActor))
  (`BloodCharacter.SetCurrentInteractable` _asbp_blood_character self))

(event `self.Box1.OnComponentEndOverlap`
  (params (OverlappedComponent :type "PrimitiveComponent Object Reference") (OtherActor :type "Actor Object Reference") (OtherComp :type "PrimitiveComponent Object Reference") (OtherBodyIndex :type Integer))
  (bind _asbp_blood_character (cast `/Game/BP/BP_BloodCharacter` OtherActor))
  (`BloodCharacter.UnsetInteractable` _asbp_blood_character self))

(event `self.SoundSphere.OnComponentBeginOverlap`
  (params (OverlappedComponent :type "PrimitiveComponent Object Reference") (OtherActor :type "Actor Object Reference") (OtherComp :type "PrimitiveComponent Object Reference") (OtherBodyIndex :type Integer) (bFromSweep :type Boolean) (SweepResult :type "HitResult Structure (by ref)"))
  (if (`self.IsOn`)
    (cast `/Game/BP/BP_BloodCharacter` OtherActor)
    (`AkGameObject.PostAkEvent` :`self` (`self.Ak`) :`AkEvent` "/Game/WwiseAudio/Events/Environment_Work_Unit/SFX_Generator_Presence.SFX_Generator_Presence")))

(event `self.SoundSphere.OnComponentEndOverlap`
  (params (OverlappedComponent :type "PrimitiveComponent Object Reference") (OtherActor :type "Actor Object Reference") (OtherComp :type "PrimitiveComponent Object Reference") (OtherBodyIndex :type Integer))
  (if (`self.IsOn`)
    (cast `/Game/BP/BP_BloodCharacter` OtherActor)
    (`AkGameObject.Stop` (`self.Ak`))))

(fn `GetOffset`
  (returns (ReturnValue :type "Float (single-precision)"))
  (return 0.0))

(fn `GetWhoCanInteract`
  (returns (ReturnValue :type "EWhoCanInteract Enum"))
  (return "ALL"))

(fn `UserConstructionScript`
  (`|ExecutionSequence`
    (:`then_0`
      (if (`self.SetObjective`)
        (set `self.ObjectiveComponent` (`self.GetComponentByClass` self "/Game/BP/Interactable/BP_Objective_AC.BP_Objective_AC_C"))))
    (:`then_1`
      (if (`self.PlayDialogue`)
        (set `self.DialogueComponent` (`self.GetComponentByClass` self "/Game/BP/Interactable/BP_Dialogue_AC.BP_Dialogue_AC_C"))))))