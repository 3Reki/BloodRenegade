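; BP_ResetSwitch is an interactable that calls ResetInteraction on its referenced Switch when used.
; An overlap box registers and unregisters it as the current interactable on BP_BloodCharacter, and its widget shows an [A] prompt.
; Interacting also flashes the cube pink, with a half-second timer restoring the basic material.
; It allows all interactors and reports a zero offset.
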(event `self.ReceiveBeginPlay`
  (set `/Game/BP/Widgets/WBP_Interact.Letter` "[A]" (cast `/Game/BP/Widgets/WBP_Interact` (`WidgetComponent.GetUserWidgetObject` (`self.Widget`)) :!pure true)))

(event `self.Interact`
  (`/Game/BP/Interactable/BP_Switch.ResetInteraction` (`self.Switch`))
  (`PrimitiveComponent.SetMaterial` (`self.Cube`) 0 "/Game/GameArt/MasterMaterial/DebugMat/MI_ColorPink.MI_ColorPink")
  (`KismetSystemLibrary.K2_SetTimerDelegate` (delegate `ResetColor`) 0.5))

(event `ResetColor`
  (`PrimitiveComponent.SetMaterial` (`self.Cube`) 0 "/Engine/BasicShapes/BasicShapeMaterial.BasicShapeMaterial"))

(event `self.Box.OnComponentBeginOverlap`
  (params (OverlappedComponent :type "PrimitiveComponent Object Reference") (OtherActor :type "Actor Object Reference") (OtherComp :type "PrimitiveComponent Object Reference") (OtherBodyIndex :type Integer) (bFromSweep :type Boolean) (SweepResult :type "HitResult Structure (by ref)"))
  (bind _asbp_blood_character (cast `/Game/BP/BP_BloodCharacter` OtherActor))
  (`BloodCharacter.SetCurrentInteractable` _asbp_blood_character self))

(event `self.Box.OnComponentEndOverlap`
  (params (OverlappedComponent :type "PrimitiveComponent Object Reference") (OtherActor :type "Actor Object Reference") (OtherComp :type "PrimitiveComponent Object Reference") (OtherBodyIndex :type Integer))
  (bind _asbp_blood_character (cast `/Game/BP/BP_BloodCharacter` OtherActor))
  (`BloodCharacter.UnsetInteractable` _asbp_blood_character self))

(fn `GetOffset`
  (returns (ReturnValue :type "Float (single-precision)"))
  (return 0.0))

(fn `GetWhoCanInteract`
  (returns (ReturnValue :type "EWhoCanInteract Enum"))
  (return "ALL"))

(fn `UserConstructionScript`)