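; Actor component that plays a Dialogue data asset's voice lines and subtitles through the player character.
; Lines run in sequence, each after its own delay, with the Wwise post-event callback advancing to the next.
; After the last line it clears subtitles and uses the owner's objective component, if present.
; PlayDialogue fires once, saved as a consumable under the owner's name, while Use skips that check.
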(event `self.ReceiveBeginPlay`
  (bind _asbp_blood_character (cast `/Game/BP/BP_BloodCharacter` (`GameplayStatics.GetPlayerCharacter` 0)))
  (set `self.As BP Blood Character` _asbp_blood_character)
  (`self.Load`)
  (set `self.ObjectiveComponent` (`Actor.GetComponentByClass` (`self.GetOwner`) "/Game/BP/Interactable/BP_Objective_AC.BP_Objective_AC_C")))

(event `PlayDialogue`
  (bind (_output_voiceline _output_subtitle _output_delaybeforevoiceline) (break `Subtitle` (`|GetArrayItem` (`SubtitleDataAsset.Subtitles` (`self.Dialogue`)) (`self.CurrentLineIndex`))))
  (if (not (`self.Activated`))
    (set `self.Activated` true)
    (message `/Game/BP/SaveSystem/BPI_Saver.SaveConsumable` (`GameplayStatics.GetGameInstance`) (`KismetSystemLibrary.GetObjectName` (`self.GetOwner`)) false)
    (`/Engine/EditorBlueprintResources/StandardMacros.IsValid` (`self.Dialogue`) :!label _label
      (:`Is Valid`
        (set `self.CurrentLineIndex` 0)
        (`KismetSystemLibrary.Delay` _output_delaybeforevoiceline :!label _label_2)
        (`AkGameObject.PostAkEvent` (`/Game/BP/BP_BloodCharacter.Ak` (`self.As BP Blood Character`)) _output_voiceline 1 (delegate `PlayNextLine`))
        (`/Game/BP/BP_BloodCharacter.AddSubtitle` (`self.As BP Blood Character`) _output_subtitle)
        (`/Engine/EditorBlueprintResources/StandardMacros.IncrementInt` (`self.CurrentLineIndex`)))
      (:`Is Not Valid`
        (`KismetSystemLibrary.PrintString` "Error: No Dialogue/Subtitles Data Asset to read" true true (struct :`R` 1.0 :`A` 1.0))))))

(event `PlayNextLine`
  (params (CallbackType :type "EAkCallbackType Enum" :default "EndOfEvent") (CallbackInfo :type "AkCallbackInfo Object Reference"))
  (bind _objectivecomponent (`self.ObjectiveComponent`))
  (if (`KismetArrayLibrary.Array_IsValidIndex` (`SubtitleDataAsset.Subtitles` (`self.Dialogue`)) (`self.CurrentLineIndex`))
    (goto _label_2)
    (else
      (`/Game/BP/Widgets/WBP_Subtitles.ClearSubtitles` (`/Game/BP/BP_BloodCharacter.Subtitles Widget` (`self.As BP Blood Character`)))
      (`/Engine/EditorBlueprintResources/StandardMacros.IsValid` _objectivecomponent
        (:`Is Valid`
          (`/Game/BP/Interactable/BP_Objective_AC.Use` _objectivecomponent))))))

(event `/Game/BP/Interactable/BPI_Activatable.Use`
  (goto _label))

(fn `Load`
  (bind (_savegamedata _saveexists) (message `/Game/BP/SaveSystem/BPI_Saver.GetSaveData` (`GameplayStatics.GetGameInstance`)))
  (if _saveexists
    (set `self.Activated` (`BlueprintSetLibrary.Set_Contains` (`/Game/BP/SaveSystem/BP_SaveGame.Consumables` _savegamedata) (`KismetSystemLibrary.GetObjectName` (`self.GetOwner`))))
    (return)
    (else
      (return))))