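; Actor component that saves and restores its owning actor's transform through save-system messages on the GameInstance.
; On BeginPlay, if a save exists, it looks up the owner's object name in the saved Actors map and teleports the owner to the stored transform.
; SaveTransform writes the current transform, shifted by a location offset, under that name without flushing the save.
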(event `self.ReceiveBeginPlay`
  (bind _returnvalue (`self.GetOwner`))
  (bind (_savegamedata _saveexists) (message `/Game/BP/SaveSystem/BPI_Saver.GetSaveData` (`GameplayStatics.GetGameInstance`)))
  (if _saveexists
    (bind (_value _returnvalue_2) (`BlueprintMapLibrary.Map_Find` (`/Game/BP/SaveSystem/BP_SaveGame.Actors` _savegamedata) (`KismetSystemLibrary.GetObjectName` _returnvalue)))
    (if _returnvalue_2
      (`Actor.K2_SetActorTransform` _returnvalue _value false true))))

(event `Save Transform`
  (params (LocationOffset :type "Vector Structure"))
  (bind _returnvalue (`self.GetOwner`))
  (message `/Game/BP/SaveSystem/BPI_Saver.SaveActor` (`GameplayStatics.GetGameInstance`) (`KismetSystemLibrary.GetObjectName` _returnvalue) (`KismetMathLibrary.MakeTransform` (+ LocationOffset (.location (`Actor.GetTransform` _returnvalue))) (.rotation (`Actor.GetTransform` _returnvalue)) (.scale (`Actor.GetTransform` _returnvalue))) false))