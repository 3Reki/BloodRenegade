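; Checkpoint actor component that saves the player's respawn point the first time a BP_BloodCharacter activates it.
; Activation fires OnActivate, then saves the respawn transform and current blood gauge fill through the game instance.
; It also records the owner's object name as a consumable, flushing both writes in that final call.
; Load restores the activated state by looking up that name in the saved consumables.
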(fn `Activate Checkpoint`
  (params (Actor :type "Actor Object Reference") (RespawnTransform :type "Transform Structure"))
  (returns (Successful :type Boolean))
  (bind _returnvalue (`GameplayStatics.GetGameInstance`))
  (if (not (`self.Activated`))
    (bind _asbp_blood_character (cast `/Game/BP/BP_BloodCharacter` Actor)
      (:`then`
        (set `self.Activated` true)
        (`self.OnActivate`)
        (bind _playersavedata (`/Game/BP/BP_BloodCharacter.GetPlayerSave` _asbp_blood_character))
        (message `/Game/BP/SaveSystem/BPI_Saver.SavePlayerData` _returnvalue (make `/Game/BP/SaveSystem/S_PlayerSaveData` (`local.RespawnTransform`) (`.BloodGaugeFill_8_C9D1BBDB47711101BE312DAA6D66276F` (break `/Game/BP/SaveSystem/S_PlayerSaveData` _playersavedata))) false)
        (message `/Game/BP/SaveSystem/BPI_Saver.SaveConsumable` _returnvalue (`KismetSystemLibrary.GetObjectName` (`self.GetOwner`)) true)
        (return true))
      (:`CastFailed`
        _)))
  (return false))

(fn `Load`
  (returns (IsActivated :type Boolean))
  (bind (_savegamedata _saveexists) (message `/Game/BP/SaveSystem/BPI_Saver.GetSaveData` (`GameplayStatics.GetGameInstance`)))
  (if _saveexists
    (bind _output_get (set `self.Activated` (`BlueprintSetLibrary.Set_Contains` (`/Game/BP/SaveSystem/BP_SaveGame.Consumables` _savegamedata) (`KismetSystemLibrary.GetObjectName` (`self.GetOwner`)))))
    (return _output_get)
    (else
      (return false))))